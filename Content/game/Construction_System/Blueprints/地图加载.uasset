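; Map loader that builds a space on the authority from a saved template and the API's NFT placement records, or only spawns check-in points on the center island.
; Template and NFT passes spawn class, glTF and FBX/OBJ objects sequentially, advancing on load callback or timeline end, with a progress widget.
; Between passes it sets embassy decals, fetches records by build/play mode and spawns play-mode check-ins.
; Over 300 model-file entries enables optimized loading.
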(event `坐标设置细节`
  (bind _returnvalue (`KismetStringLibrary.Conv_StringToInt` (`/Game/game/INS.加入的空间坐标` (cast `/Game/game/INS` (`GameplayStatics.GetGameInstance`) :!pure true))))
  (bind _returnvalue_2 (`KismetArrayLibrary.Array_Find` (`self.大使馆的坐标`) _returnvalue))
  (if (> _returnvalue 12)
    (if (>= _returnvalue_2 0)
      (bind _outactors (`GameplayStatics.GetAllActorsOfClass` "/Game/game/blueprint/Decoration/贴花系统.贴花系统_C"))
      (`/Game/game/blueprint/Decoration/贴花系统.设置贴图` (`|GetArrayItem` _outactors) (select `int` _returnvalue_2 :`0` "/Game/ZY/静态网格体/RacingFlagsMegaBundle/Meshes/阿拉伯.阿拉伯" :`1` "/Game/ZY/静态网格体/RacingFlagsMegaBundle/Meshes/印度.印度" :`2` "/Game/ZY/静态网格体/RacingFlagsMegaBundle/Meshes/印度尼西亚.印度尼西亚" :`3` "/Game/ZY/静态网格体/RacingFlagsMegaBundle/Meshes/尼日利亚.尼日利亚" :`4` "/Game/ZY/静态网格体/RacingFlagsMegaBundle/Meshes/摩洛哥.摩洛哥" :`5` "/Game/ZY/静态网格体/RacingFlagsMegaBundle/Meshes/英国.英国" :`6` "/Game/ZY/静态网格体/RacingFlagsMegaBundle/Meshes/法国.法国" :`7` "/Game/ZY/静态网格体/RacingFlagsMegaBundle/Meshes/乌克兰.乌克兰" :`8` "/Game/ZY/静态网格体/RacingFlagsMegaBundle/Meshes/俄罗斯.俄罗斯" :`9` "/Game/ZY/静态网格体/RacingFlagsMegaBundle/Meshes/越南.越南" :`10` "/Game/ZY/静态网格体/RacingFlagsMegaBundle/Meshes/菲律宾.菲律宾" :`11` "/Game/ZY/静态网格体/RacingFlagsMegaBundle/Meshes/澳大利亚.澳大利亚" :`12` "/Game/ZY/静态网格体/RacingFlagsMegaBundle/Meshes/墨西哥.墨西哥" :`13` "/Game/ZY/静态网格体/RacingFlagsMegaBundle/Meshes/美国.美国" :`14` "/Game/ZY/静态网格体/RacingFlagsMegaBundle/Meshes/加拿大.加拿大" :!type "Texture Object Reference")))))

(event `生成打卡点`
  (bind _asins (cast `/Game/game/INS` (`GameplayStatics.GetGameInstance`) :!pure true))
  (if (not (`/Game/game/函数库.为建造模式`))
    (bind _returnvalue (`VaRestSubsystem.ConstructVaRestRequestExt` (subsystem `VaRestSubsystem`) "GET" "x_www_form_urlencoded_url"))
    (`VaRestRequestJSON.SetHeader` _returnvalue "X-Access-Token" (`/Game/game/INS.令牌` _asins))
    (`VaRestRequestJSON.ProcessURL` _returnvalue (`/Game/game/函数库.附加区块链接口` (`KismetStringLibrary.Concat_StrStr` (`/Game/game/INS.API` _asins) "mgn/islandAirdrop/list?status=0x01&pageSize=-1")))
    (add `VaRestRequestJSON.OnRequestComplete` _returnvalue (delegate `打卡点数据返回`))))

(event `打卡点数据返回`
  (params (Request :type "VaRestRequestJSON Object Reference"))
  (bind `_打卡点json` (`self.打卡点json`))
  (bind _returnvalue (`KismetStringLibrary.Conv_StringToInt` (`/Game/game/INS.加入的空间坐标` (cast `/Game/game/INS` (`GameplayStatics.GetGameInstance`) :!pure true))))
  (set `self.打卡点json` (`|MakeJson`))
  (bind _returnvalue_2 (`VaRestRequestJSON.GetResponseContentAsString` Request false))
  (`VaRestJsonObject.DecodeJson` `_打卡点json` _returnvalue_2 false)
  (for _array_element (`VaRestJsonObject.GetObjectArrayField` (`VaRestJsonObject.GetObjectField` `_打卡点json` "result") "records")
    (if (== (`VaRestJsonObject.GetIntegerField` (`VaRestJsonObject.GetObjectField` _array_element "island") "coordinate") _returnvalue)
      (bind (_structarray _returnvalue_3) (`JsonCsvToDataTableToStructBPLibrary.JsonStringToStructArrayV2` (`VaRestJsonObject.GetStringField` _array_element "airdropConfig")))
      (if _returnvalue_3
        (bind _returnvalue_4 (`GameplayStatics.GetCurrentLevelName` true))
        (bind (_lefts _rights) (`KismetStringLibrary.Split` _returnvalue_4 "MB"))
        (bind (_lefts_2 _rights_2 _returnvalue_5) (`KismetStringLibrary.Split` _rights "JZ"))
        (bind _returnvalue_6 (- (select `bool` _returnvalue_5 :`false` (`KismetStringLibrary.Conv_StringToInt` _rights) :`true` (`KismetStringLibrary.Conv_StringToInt` _lefts_2)) 1))
        (bind _output (`|GetArrayItem` _structarray (select `bool` (== _returnvalue 0) :`false` (select `bool` (< _returnvalue_6 0) :`false` _returnvalue_6))))
        (bind (_baselink _baselocation _baserotate) (break `/Game/game/结构/空投结构` _output))
        (`|SpawnActorFromClass` :`Class` "/Game/game/blueprint/Interactive_Object/打卡点.打卡点_C" :`SpawnTransform` (`KismetMathLibrary.MakeTransform` _baselocation (`/Game/game/函数库.向量转旋转` _baserotate)) :`CollisionHandlingOverride` "AlwaysSpawn" :`TransformScaleMethod` "MultiplyWithRoot" :`空投结构` _output :`islandAirdropId` (`VaRestJsonObject.GetIntegerField` _array_element "islandAirdropId") :`blockchainId` (`VaRestJsonObject.GetStringField` _array_element "blockchainId") :`Asset` null :`Instigator` null)))))

(event `self.ReceiveBeginPlay`
  (bind `_gltf数量` (`self.GLTF数量`))
  (bind `_建造空间路径` (`/Game/game/INS.建造空间路径` (cast `/Game/game/INS` (`GameplayStatics.GetGameInstance`) :!pure true)))
  (`KismetSystemLibrary.Delay` 0.2)
  (set `self.建造模式` (`/Game/game/函数库.为建造模式`))
  (`/Engine/EditorBlueprintResources/ActorMacros.Switch Has Authority`
    (:`Authority`
      (if (`self.为中心岛`)
        (`self.生成打卡点`)
        (elif (not (`KismetStringLibrary.IsEmpty` `_建造空间路径`))
          (bind _structarray (`JsonCsvToDataTableToStructBPLibrary.JsonStringToStructArrayV2` (`FileSDKBPLibrary.ReadStringFromFile` (`KismetStringLibrary.Concat_StrStr` (`/Game/game/函数库.获取MAP路径`) `_建造空间路径`))))
          (bind _output_get (set `self.actor结构` _structarray))
          (set `self.加载数量` (`KismetArrayLibrary.Array_Length` _output_get))
          (for _array_element (`self.actor结构`)
            (if (not (`KismetStringLibrary.IsEmpty` (`.GLTF_path_67_D9C640E34A9BA5140AE848A53C4CC2D5` (break `/Game/game/结构/建造结构/Actor_structure` _array_element))))
              (`/Engine/EditorBlueprintResources/StandardMacros.IncrementInt` `_gltf数量`)))
          (set `self.启用优化加载` (> `_gltf数量` 300))
          (if (> (`self.加载数量`) 0)
            (bind _outactors (`GameplayStatics.GetAllActorsOfClass` "/Game/game/blueprint/Interactive_Object/General_category_objects.General_category_objects_C"))
            (for _array_element_2 _outactors
              (if (`|EnumEquality` (`/Game/game/blueprint/Interactive_Object/General_category_objects.生成状态枚举` _array_element_2) "NewEnumerator0")
                (`self.K2_DestroyActor` _array_element_2)))
            (`KismetSystemLibrary.Delay` 0.5)
            (`self.生成物体` 1)))))))

(event `生成物体`
  (params (`1模板生成2nft生成` :type Integer))
  (bind `_生成索引` (`self.生成索引`))
  (bind `_生成索引_2` (`self.生成索引`))
  (bind `_生成索引_3` (`self.生成索引`))
  (bind `_生成索引_4` (`self.生成索引`))
  (bind `_生成索引_5` (`self.生成索引`))
  (bind _output (`|GetArrayItem` (`self.actor结构`) `_生成索引_5`))
  (bind _returnvalue (- (`self.加载数量`) 1))
  (bind (_transform _id _gltf_path _interaction _image_link _animation_path _actor_class) (break `/Game/game/结构/建造结构/Actor_structure` _output))
  (bind _b1 (`/Game/game/函数库.变换转变换` _transform))
  (bind _returnvalue_2 (== (`KismetStringLibrary.GetSubstring` _gltf_path (- (`KismetStringLibrary.Len` _gltf_path) 3) 3) "glb"))
  (set `self.1模板生成2nft生成` `1模板生成2nft生成`)
  (set `self.生成索引` 0)
  (bind `_加载控件` (`self.加载控件` :!label _label)
    (:`then`
      (set `/Game/game/控件/加载提示控件.进度` (`KismetMathLibrary.FTrunc` (* (/ (`KismetMathLibrary.Conv_IntToDouble` (`self.生成索引`)) (`KismetMathLibrary.Conv_IntToDouble` _returnvalue)) 100.0)) `_加载控件`))
    (:`else`
      (bind _returnvalue_3 (`|CreateWidget` "/Game/game/控件/加载提示控件.加载提示控件_C" null "Loading…"))
      (`UserWidget.AddToViewport` _returnvalue_3 0)
      (set `self.加载控件` _returnvalue_3)))
  (if (> `_生成索引_5` _returnvalue)
    (set `self.空间摆放json` null)
    (set `self.材质json` null)
    (`KismetArrayLibrary.Array_Clear` (`self.actor结构`))
    (switch `int` (`self.1模板生成2nft生成`)
      (:`1`
        (`self.坐标设置细节`)
        (`self.获取空间摆放NFT`)
        (`self.生成打卡点`))
      (:`2`
        (`Widget.RemoveFromParent` (`self.加载控件`))
        (bind _outactors (`GameplayStatics.GetAllActorsOfClass` "/Game/game/blueprint/Interactive_Object/General_category_objects.General_category_objects_C"))
        (for _array_element _outactors
          (`/Game/game/blueprint/Interactive_Object/General_category_objects.场景加载完毕` _array_element))))
    (else
      (bind _struct (`JsonCsvToDataTableToStructBPLibrary.JsonStringToStructV2` _actor_class))
      (bind _output_get (set `self.actor类` _struct))
      (switch `int` (`self.1模板生成2nft生成`)
        (:`1`
          (if (== (.location (`/Game/game/函数库.变换转变换` _transform)) (0.0 0.0 0.0))
            ;[1 1 1] 跳过原点物体生成
            (`self.加载下一个`)
            (else
              (`|ExecutionSequence` :!label _label_2
                (:`then_0`
                  (goto _label_4 :!via `Reset`))
                (:`then_1`
                  (if (`KismetStringLibrary.IsEmpty` _gltf_path)
                    (bind _actor_class_2 (break `/Game/game/结构/建造结构/Actor_class_structure` _output_get))
                    (bind _asgeneral_category_objects (castclass `/Game/game/blueprint/Interactive_Object/General_category_objects` _actor_class_2)
                      (:`then`
                        ;[1 1 1] 其他
                        (bind _returnvalue_4 (`|SpawnActorFromClass` :`Class` _asgeneral_category_objects :`SpawnTransform` _b1 :`CollisionHandlingOverride` "AlwaysSpawn" :`TransformScaleMethod` "SelectDefaultAtRuntime" :`NFTid` (select `int` (`self.1模板生成2nft生成`) :`0` "" :`1` "" :`2` (`|GetArrayItem` (`self.NFTID`) `_生成索引_2`)) :`actor摆放结构` _output :`场景ID` (select `int` (`self.1模板生成2nft生成`) :`0` "" :`1` "" :`2` (`|GetArrayItem` (`self.场景ID`) `_生成索引_2`)) :`生成状态枚举` "NewEnumerator1" :`优化加载` (`self.启用优化加载`) :`Asset` null :`Instigator` null))
                        (add `/Game/game/blueprint/Interactive_Object/General_category_objects.加载完毕` _returnvalue_4 (delegate `绑定1`))
                        (`/Game/game/blueprint/Interactive_Object/General_category_objects.加载绑定完成` _returnvalue_4)
                        (`Timeline|时间轴` :!via `PlayFromStart` :!label _label_3
                          (:`Finished`
                            (`/Engine/EditorBlueprintResources/StandardMacros.DoOnce` false :!label _label_4
                              (:`Completed`
                                (`KismetSystemLibrary.Delay` 0.02)
                                (`/Engine/EditorBlueprintResources/StandardMacros.IncrementInt` (`self.生成索引`) :!label _label_5
                                  (:`  `
                                    (goto _label))))))))
                      (:`CastFailed`
                        (bind `_as自定义可交互物` (castclass `/Game/game/blueprint/Agent可交互物/自定义可交互物` _actor_class_2)
                          (:`then`
                            (bind _returnvalue_5 (`|SpawnActorFromClass` :`Class` `_as自定义可交互物` :`SpawnTransform` _b1 :`CollisionHandlingOverride` "AlwaysSpawn" :`TransformScaleMethod` "MultiplyWithRoot" :`actor摆放结构` (`|GetArrayItem` (`self.actor结构`) (`self.生成索引`)) :`Instigator` null))
                            (`/Game/game/blueprint/Agent可交互物/自定义可交互物.地图生成初始化` _returnvalue_5 (`self.建造模式`)))
                          (:`CastFailed`
                            _))
                        (`|ExecutionSequence` :!label _label_6
                          (:`then_0`
                            (goto _label_3 :!via `Stop`))
                          (:`then_1`
                            (goto _label_4)))))
                    (else
                      (if (`self.启用优化加载`)
                        (if _returnvalue_2
                          ;[1 1 1] gltf导入
                          (`|SpawnActorFromClass` :`Class` "/Game/game/blueprint/Interactive_Object/GLTF/GLTF导入.GLTF导入_C" :`SpawnTransform` (`KismetMathLibrary.MakeTransform` (.location _b1) (.rotation _b1) (.scale _b1)) :`CollisionHandlingOverride` "AlwaysSpawn" :`TransformScaleMethod` "MultiplyWithRoot" :`NFTid` (select `int` (`self.1模板生成2nft生成`) :`0` "" :`1` "" :`2` (`|GetArrayItem` (`self.NFTID`) `_生成索引_3`)) :`actor摆放结构` _output :`场景ID` (select `int` (`self.1模板生成2nft生成`) :`0` "" :`1` "" :`2` (`|GetArrayItem` (`self.场景ID`) `_生成索引_3`)) :`生成状态枚举` "NewEnumerator1" :`优化加载` true :`Asset` null :`Instigator` null)
                          (goto _label_6)
                          (else
                            _))
                        (elif _returnvalue_2
                          (bind _returnvalue_6 (`glTFRuntimeFunctionLibrary.glTFLoadAssetFromFilename` (`KismetStringLibrary.Concat_StrStr` (`/Game/game/函数库.Gltf路径` true) _gltf_path) false (make `glTFRuntimeConfig` "YForward")))
                          ;[1 1 1] gltf
                          (bind _returnvalue_7 (`|SpawnActorFromClass` :`Class` _asgeneral_category_objects :`SpawnTransform` _b1 :`CollisionHandlingOverride` "AlwaysSpawn" :`TransformScaleMethod` "SelectDefaultAtRuntime" :`NFTid` (select `int` (`self.1模板生成2nft生成`) :`0` "" :`1` "" :`2` (`|GetArrayItem` (`self.NFTID`) `_生成索引_4`)) :`actor摆放结构` _output :`场景ID` (select `int` (`self.1模板生成2nft生成`) :`0` "" :`1` "" :`2` (`|GetArrayItem` (`self.场景ID`) `_生成索引_4`)) :`生成状态枚举` "NewEnumerator1" :`Asset` _returnvalue_6 :`StaticMeshConfig` (make `glTFRuntimeStaticMeshConfig` :`bBuildSimpleCollision` true :`bBuildComplexCollision` true :`CollisionComplexity` "CTF_UseComplexAsSimple" :`bAllowCPUAccess` true) :`Instigator` null))
                          (add `/Game/game/blueprint/Interactive_Object/General_category_objects.加载完毕` _returnvalue_7 (delegate `绑定2`))
                          (`/Game/game/blueprint/Interactive_Object/General_category_objects.加载绑定完成` _returnvalue_7)
                          (goto _label_3 :!via `PlayFromStart`)
                          (else
                            _)))
                      ;[1 1 1] fbx_Obj
                      (bind _returnvalue_8 (`|SpawnActorFromClass` :`Class` "/Game/game/blueprint/Interactive_Object/FBX/Fbx_Obj.Fbx_Obj_C" :`SpawnTransform` _b1 :`CollisionHandlingOverride` "AlwaysSpawn" :`TransformScaleMethod` "MultiplyWithRoot" :`NFTid` (select `int` (`self.1模板生成2nft生成`) :`0` "" :`1` "" :`2` (`|GetArrayItem` (`self.NFTID`) `_生成索引`)) :`actor摆放结构` _output :`场景ID` (select `int` (`self.1模板生成2nft生成`) :`0` "" :`1` "" :`2` (`|GetArrayItem` (`self.场景ID`) `_生成索引`)) :`生成状态枚举` "NewEnumerator1" :`优化加载` (`self.启用优化加载`) :`Asset` null :`Instigator` null))
                      (add `/Game/game/blueprint/Interactive_Object/General_category_objects.加载完毕` _returnvalue_8 (delegate `绑定3`))
                      (`/Game/game/blueprint/Interactive_Object/General_category_objects.加载绑定完成` _returnvalue_8)
                      (goto _label_3 :!via `PlayFromStart`))))))))
        (:`2`
          (goto _label_2))))))

(event `加载下一个`
  (goto _label_5))

(event `绑定1`
  (goto _label_6))

(event `获取空间摆放NFT`
  (bind _asins (cast `/Game/game/INS` (`GameplayStatics.GetGameInstance`) :!pure true))
  (bind _asins_2 (cast `/Game/game/INS` (`GameplayStatics.GetGameInstance`) :!pure true))
  (`KismetArrayLibrary.Array_Clear` (`self.actor结构`))
  (set `self.当前页数` 1)
  (set `self.空间摆放json` (`|MakeJson`))
  (set `self.材质json` (`|MakeJson`))
  (if (`self.建造模式`)
    (bind _returnvalue (`VaRestSubsystem.ConstructVaRestRequestExt` (subsystem `VaRestSubsystem`) "GET" "x_www_form_urlencoded_url" :!label _label_7))
    (`VaRestRequestJSON.SetHeader` _returnvalue "X-Access-Token" (`/Game/game/INS.令牌` _asins))
    (`VaRestRequestJSON.ProcessURL` _returnvalue (`/Game/game/函数库.附加区块链接口` (`KismetStringLibrary.Concat_StrStr` (`/Game/game/INS.API` _asins) "mgn/nftPlaceRecord/list?pageSize=100&pageNo=" (`KismetStringLibrary.Conv_IntToString` (`self.当前页数`)) "&sid=" (`/Game/game/INS.加入的模板空间SID` _asins))))
    (add `VaRestRequestJSON.OnRequestComplete` _returnvalue (delegate `模型信息返回`))
    (else
      (bind _returnvalue_2 (`VaRestSubsystem.ConstructVaRestRequestExt` (subsystem `VaRestSubsystem`) "GET" "x_www_form_urlencoded_url"))
      (`VaRestRequestJSON.ProcessURL` _returnvalue_2 (`/Game/game/函数库.附加区块链接口` (`KismetStringLibrary.Concat_StrStr` (`/Game/game/INS.API` _asins_2) "mgn/nftPlaceRecord/getNftPlaceRecordList?sid=" (`/Game/game/INS.最近加入的空间SID` _asins_2))))
      (add `VaRestRequestJSON.OnRequestComplete` _returnvalue_2 (delegate `链上摆放记录返回`)))))

(event `绑定2`
  (goto _label_6))

(event `模型信息返回`
  (params (Request :type "VaRestRequestJSON Object Reference"))
  (bind `_空间摆放json` (`self.空间摆放json`))
  (bind `_当前页数` (`self.当前页数`))
  (bind `_材质json` (`self.材质json`))
  (bind _returnvalue (`VaRestJsonObject.GetObjectField` `_空间摆放json` "result"))
  (bind _returnvalue_2 (`VaRestRequestJSON.GetResponseContentAsString` Request false))
  (`VaRestJsonObject.DecodeJson` `_空间摆放json` _returnvalue_2 false)
  (for _array_element (`VaRestJsonObject.GetObjectArrayField` _returnvalue "records")
    (bind _returnvalue_3 (`VaRestJsonObject.GetStringField` _array_element "scenesData"))
    (bind _struct (`JsonCsvToDataTableToStructBPLibrary.JsonStringToStructV2` _returnvalue_3))
    (set `self.actor单个结构` _struct)
    (if (not (`KismetStringLibrary.IsEmpty` (`.Actor_class_72_7AA446724BEC4B342576AEAED3BFB418` (break `/Game/game/结构/建造结构/Actor_structure` (`self.actor单个结构`)))))
      (`VaRestJsonObject.DecodeJson` `_材质json` _returnvalue_3 true)
      (for (_array_element_2 _array_index) (`VaRestJsonObject.GetObjectArrayField` `_材质json` "material")
        (if (not (> (`KismetStringLibrary.Len` (`VaRestJsonObject.EncodeJsonToSingleString` _array_element_2)) 20))
          (`KismetArrayLibrary.Array_Set` (`.Material_73_4539C4174389973FC9FBF3AD6D523F76` (break `/Game/game/结构/建造结构/Actor_structure` (`self.actor单个结构`))) _array_index (make `/Game/game/Construction_System/Material_System/Material_system_structure` "") true)))
      (`KismetArrayLibrary.Array_Add` (`self.actor结构`) (`self.actor单个结构`))
      (`KismetArrayLibrary.Array_Add` (`self.NFTID`) (`VaRestJsonObject.GetStringField` _array_element "nftId"))
      (`KismetArrayLibrary.Array_Add` (`self.场景ID`) (`VaRestJsonObject.GetStringField` _array_element "recordId"))))
  (if (>= `_当前页数` (`VaRestJsonObject.GetIntegerField` _returnvalue "pages"))
    (set `self.加载数量` (`KismetArrayLibrary.Array_Length` (`self.actor结构`)))
    (`self.生成物体` 2)
    (else
      (`KismetSystemLibrary.Delay` 0.2)
      (`/Engine/EditorBlueprintResources/StandardMacros.IncrementInt` `_当前页数`
        (:`  `
          (set `self.空间摆放json` null)
          (goto _label_7))))))

(event `绑定3`
  (goto _label_6))

(event `链上摆放记录返回`
  (params (Request :type "VaRestRequestJSON Object Reference"))
  (bind `_空间摆放json` (`self.空间摆放json`))
  (bind `_材质json` (`self.材质json`))
  (bind _asins (cast `/Game/game/INS` (`GameplayStatics.GetGameInstance`) :!pure true))
  (bind _returnvalue (`VaRestRequestJSON.GetResponseContentAsString` Request false))
  (`VaRestJsonObject.DecodeJson` `_空间摆放json` _returnvalue false)
  (for _array_element (`VaRestJsonObject.GetObjectArrayField` `_空间摆放json` "result")
    (bind _returnvalue_2 (`VaRestJsonObject.GetStringField` _array_element "scenesData"))
    (bind _struct (`JsonCsvToDataTableToStructBPLibrary.JsonStringToStructV2` _returnvalue_2))
    (set `self.actor单个结构` _struct)
    (if (not (`KismetStringLibrary.IsEmpty` (`.Actor_class_72_7AA446724BEC4B342576AEAED3BFB418` (break `/Game/game/结构/建造结构/Actor_structure` (`self.actor单个结构`)))))
      (`VaRestJsonObject.DecodeJson` `_材质json` _returnvalue_2 true)
      (for (_array_element_2 _array_index) (`VaRestJsonObject.GetObjectArrayField` `_材质json` "material")
        (if (not (> (`KismetStringLibrary.Len` (`VaRestJsonObject.EncodeJsonToSingleString` _array_element_2)) 20))
          (`KismetArrayLibrary.Array_Set` (`.Material_73_4539C4174389973FC9FBF3AD6D523F76` (break `/Game/game/结构/建造结构/Actor_structure` (`self.actor单个结构`))) _array_index (make `/Game/game/Construction_System/Material_System/Material_system_structure` "") true)))
      (`KismetArrayLibrary.Array_Add` (`self.actor结构`) (`self.actor单个结构`))
      (`KismetArrayLibrary.Array_Add` (`self.NFTID`) (`VaRestJsonObject.GetStringField` _array_element "nftId"))
      (`KismetArrayLibrary.Array_Add` (`self.场景ID`) (`VaRestJsonObject.GetStringField` _array_element "recordId"))))
  (bind _returnvalue_3 (`VaRestSubsystem.ConstructVaRestRequestExt` (subsystem `VaRestSubsystem`) "GET" "x_www_form_urlencoded_url" :!label _label_8))
  (`VaRestRequestJSON.SetHeader` _returnvalue_3 "X-Access-Token" (`/Game/game/INS.令牌` _asins))
  (`VaRestRequestJSON.ProcessURL` _returnvalue_3 (`/Game/game/函数库.附加区块链接口` (`KismetStringLibrary.Concat_StrStr` (`/Game/game/INS.API` _asins) "mgn/nftPlaceRecord/list?pageSize=100&pageNo=" (`KismetStringLibrary.Conv_IntToString` (`self.当前页数`)) "&sid=" (`/Game/game/INS.最近加入的空间SID` _asins))))
  (add `VaRestRequestJSON.OnRequestComplete` _returnvalue_3 (delegate `游玩模式摆放生成`)))

(event `摆放记录返回`
  (params (Request :type "VaRestRequestJSON Object Reference"))
  (bind `_空间摆放json` (`self.空间摆放json`))
  (bind _asplay (cast `/Game/game/PLAY` (`GameplayStatics.GetPlayerController` 0) :!pure true))
  (bind _returnvalue (`VaRestJsonObject.GetStringField` (`|GetArrayItem` (`VaRestJsonObject.GetObjectArrayField` (`VaRestJsonObject.GetObjectField` `_空间摆放json` "result") "records")) "placementRecord"))
  (bind _returnvalue_2 (`VaRestRequestJSON.GetResponseContentAsString` Request false))
  (`VaRestJsonObject.DecodeJson` `_空间摆放json` _returnvalue_2 false)
  (add `/Game/game/PLAY.解压完成返回内容` _asplay (delegate `解压摆放记录`))
  (if (`KismetStringLibrary.IsEmpty` _returnvalue)
    (`self.生成物体` 2)
    (else
      (`/Game/game/PLAY.解压文件` _asplay (`KismetStringLibrary.Concat_StrStr` "data:application/json;base64," _returnvalue)))))

(event `解压摆放记录`
  (params (`内容` :type String))
  (for _array_element (`.String Array` (`|JsonToArray` `内容`))
    (bind (_success _scenesdata _nftid _recordid) (`|Json` _array_element))
    (bind _struct (`JsonCsvToDataTableToStructBPLibrary.JsonStringToStructV2` _scenesdata))
    (`KismetArrayLibrary.Array_Add` (`self.actor结构`) _struct)
    (`KismetArrayLibrary.Array_Add` (`self.NFTID`) _nftid)
    (`KismetArrayLibrary.Array_Add` (`self.场景ID`) _recordid))
  (goto _label_8))

(event `游玩模式摆放生成`
  (params (Request :type "VaRestRequestJSON Object Reference"))
  (bind `_空间摆放json` (`self.空间摆放json`))
  (bind `_当前页数` (`self.当前页数`))
  (bind _returnvalue (`VaRestJsonObject.GetObjectField` `_空间摆放json` "result"))
  (bind _returnvalue_2 (`VaRestRequestJSON.GetResponseContentAsString` Request false))
  (`VaRestJsonObject.DecodeJson` `_空间摆放json` _returnvalue_2 false)
  (for _array_element (`VaRestJsonObject.GetObjectArrayField` _returnvalue "records")
    (bind _struct (`JsonCsvToDataTableToStructBPLibrary.JsonStringToStructV2` (`VaRestJsonObject.GetStringField` _array_element "scenesData")))
    (bind _struct_2 (`JsonCsvToDataTableToStructBPLibrary.JsonStringToStructV2` (`.Actor_class_72_7AA446724BEC4B342576AEAED3BFB418` (break `/Game/game/结构/建造结构/Actor_structure` _struct))))
    (bind _actor_class (break `/Game/game/结构/建造结构/Actor_class_structure` _struct_2))
    (castclass `/Game/game/blueprint/Interactive_Object/Vehicle/Vehicle_Binding` _actor_class
      (:`then`
        _)
      (:`CastFailed`
        (castclass `/Game/game/ChenSong/音乐播放器/蓝图/Music_player` _actor_class)))
    (`KismetArrayLibrary.Array_Add` (`self.actor结构`) _struct)
    (`KismetArrayLibrary.Array_Add` (`self.NFTID`) (`VaRestJsonObject.GetStringField` _array_element "nftId"))
    (`KismetArrayLibrary.Array_Add` (`self.场景ID`) (`VaRestJsonObject.GetStringField` _array_element "recordId")))
  (if (>= `_当前页数` (`VaRestJsonObject.GetIntegerField` _returnvalue "pages"))
    (set `self.加载数量` (`KismetArrayLibrary.Array_Length` (`self.actor结构`)))
    (`self.生成物体` 2)
    (else
      (`KismetSystemLibrary.Delay` 0.2)
      (`/Engine/EditorBlueprintResources/StandardMacros.IncrementInt` `_当前页数`
        (:`  `
          (goto _label_8))))))

(fn `UserConstructionScript`)