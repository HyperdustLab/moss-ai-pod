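; Actor that drives a Niagara trail effect from the transform of a static mesh, with a spline and timeline set up for path movement.
; Each Tick it passes the mesh's world location and forward-vector-derived quaternion to the OriginLocation and OriginRotator Niagara variables.
; The Construction Script seeds both variables from the actor transform.
; The nodes that move the mesh along the spline and set the timeline rate never run.
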(event `self.ReceiveBeginPlay`)

(event `self.ReceiveTick`
  (params (DeltaSeconds :type "Float (single-precision)"))
  (bind _staticmesh (`self.StaticMesh`))
  (`NiagaraComponent.SetNiagaraVariableVec3` (`self.Niagara`) "OriginLocation" (`SceneComponent.K2_GetComponentLocation` _staticmesh))
  (`NiagaraComponent.SetNiagaraVariableQuat` (`self.Niagara`) "OriginRotator" (`KismetMathLibrary.Conv_VectorToQuaternion` (`KismetMathLibrary.GetForwardVector` (`SceneComponent.K2_GetComponentRotation` _staticmesh)))))

(fn `UserConstructionScript`
  (`NiagaraComponent.SetNiagaraVariableVec3` (`self.Niagara`) "OriginLocation" (`self.K2_GetActorLocation`))
  (`NiagaraComponent.SetNiagaraVariableQuat` (`self.Niagara`) "OriginRotator" (`KismetMathLibrary.Conv_VectorToQuaternion` (`KismetMathLibrary.GetForwardVector` (`self.K2_GetActorRotation`)))))