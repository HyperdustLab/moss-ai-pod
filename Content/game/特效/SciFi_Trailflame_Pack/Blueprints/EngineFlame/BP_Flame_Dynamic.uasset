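; BP_Flame_Dynamic is an example engine-flame actor from the SciFi Trailflame pack that varies its Niagara effect at runtime.
; Tick runs through a Delay, so updates land roughly every 0.2 seconds rather than every frame.
; Each update sets the User.AirColor parameter from scaled random unit-vector components and User.AirLength from a random integer range, changing the flame's color and length.
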(event `self.ReceiveTick`
  (params (DeltaSeconds :type "Float (single-precision)"))
  ;[1 1 1] ExampleOfDynamicFlame
  (`parent.ReceiveTick` DeltaSeconds)
  (`KismetSystemLibrary.Delay` 0.2)
  (`NiagaraComponent.SetNiagaraVariableLinearColor` (`self.Niagara`) "User.AirColor" (make `LinearColor` (.x (* (`KismetMathLibrary.RandomUnitVector`) (`KismetMathLibrary.RandomIntegerInRange` 10 11))) (.y (* (`KismetMathLibrary.RandomUnitVector`) (`KismetMathLibrary.RandomIntegerInRange` 10 11))) (.z (* (`KismetMathLibrary.RandomUnitVector`) (`KismetMathLibrary.RandomIntegerInRange` 10 11))) 1.0))
  (`NiagaraComponent.SetNiagaraVariableFloat` (`self.Niagara`) "User.AirLength" (`KismetMathLibrary.Conv_IntToDouble` (`KismetMathLibrary.RandomIntegerInRange` 1000 3000))))

(fn `UserConstructionScript`
  (`parent.UserConstructionScript`))