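; Data-driven custom interactable that players place in build mode and AI Agents use to perform named actions.
; Actions are saved with transform, class and IDs as JSON in the placement structure, then restored on map generation.
; Interaction matches the requested action, posts it to chat, and plays enter/sustain or leave montages along a spline.
; Delay-polling waits on animations before applying attribute changes (enter actions only) and completing the Agent's node.
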(event `物体收起`
  (params (`收起` :type Boolean :default true))
  (set `self.actor已收起` `收起`)
  (`|ExecutionSequence`
    (:`then_0`
      (`self.SetActorHiddenInGame` `收起`)
      (`self.SetActorEnableCollision` (not `收起`))
      (set `self.保存时忽略` `收起`))))

(event `摆放初始化`
  (params (`摆放json数据` :type "VaRestJsonObject Object Reference") (`随机ID` :type String))
  (bind `_建造模型点击` (`self.建造模型点击`))
  (set `self.场景ID` `随机ID`)
  (set `self.NFTID` (`VaRestJsonObject.GetStringField` `摆放json数据` "id"))
  ;[1 1 1] 显示模型点击
  (`SceneComponent.SetVisibility` `_建造模型点击` true false :!label _label)
  (`PrimitiveComponent.SetCollisionEnabled` `_建造模型点击` "QueryAndPhysics"))

(event `地图生成初始化`
  (params (`为建造模式` :type Boolean))
  (bind (_transform _id _gltf_path _interaction _image_link _animation_path _actor_class _material _boolean _float _character) (break `/Game/game/结构/建造结构/Actor_structure` (`self.actor摆放结构`)))
  (`|ExecutionSequence`
    (:`then_0`
      (bind _output_get (set `self.为建造模式` `为建造模式`))
      (if _output_get
        (goto _label)))
    (:`then_1`
      (set `self.NFTID` _id)
      (set `self.场景ID` (`|GetArrayItem` _character 1))
      (bind _structarray (`JsonCsvToDataTableToStructBPLibrary.JsonStringToStructArrayV2` (`|GetArrayItem` _character)))
      (bind _output_get_2 (set `self.自定义交互物结构` _structarray))
      (for _array_element _output_get_2
        (`KismetArrayLibrary.Array_Add` (`self.所有参数`) (`.动作_7_2642A6D0444B5CFD19D0ABB180145703` (break `/Game/game/结构/Agent/自定义交互物结构` _array_element)))))))

(event `保存至摆放结构`
  (bind _output_get (set `self.actor类结构` (make `/Game/game/结构/建造结构/Actor_class_structure` (`GameplayStatics.GetObjectClass` self))))
  (bind _outjsonstring (`JsonCsvToDataTableToStructBPLibrary.StructToJsonObjectString` _output_get))
  (bind _outjsonstring_2 (`JsonCsvToDataTableToStructBPLibrary.StructArrayToJsonObjectStringV2` (`self.自定义交互物结构`)))
  (set `self.actor摆放结构` (make `/Game/game/结构/建造结构/Actor_structure` :`Transform` (`.B2` (`/Game/game/函数库.变换转变换` (struct) (`self.GetTransform`))) :`ID` (`self.NFTID`) :`Actor_class` (`/Game/game/函数库.去除json换行符` _outjsonstring) :`Character` (`|MakeArray` _outjsonstring_2 (`self.场景ID`)))))

(event `self.执行交互`
  (bind `_正在交互的agent` (`self.正在交互的Agent`))
  (bind `_正在交互的agent_2` (`self.正在交互的Agent`))
  (bind (`_名称` `_提示词` `_动作` `_交互位置` `_进入动画` `_持续动画` `_离开动画` `_属性变更规则`) (break `/Game/game/结构/Agent/自定义交互物结构` (`self.当前找到的动作`)))
  (bind (`_名称_2` `_提示词_2` `_动作_2` `_交互位置_2` `_进入动画_2`) (break `/Game/game/结构/Agent/自定义交互物结构` (`self.当前找到的动作`)))
  (bind (`_名称_3` `_提示词_3` `_动作_3` `_交互位置_3` `_进入动画_3` `_持续动画_2` `_离开动画_2`) (break `/Game/game/结构/Agent/自定义交互物结构` (`self.当前找到的动作`)))
  (bind (`_名称_4` `_提示词_4` `_动作_4` `_交互位置_4` `_进入动画_4` `_持续动画_3` `_离开动画_3` `_属性变更规则_2`) (break `/Game/game/结构/Agent/自定义交互物结构` (`self.当前找到的动作`)))
  (bind (_mood _money _reputation _creativity _emotion _charm _knowledge _strength) (break `/Game/game/结构/Agent/Agent模拟属性` `_属性变更规则`))
  (bind (_mood_2 _money_2 _reputation_2 _creativity_2 _emotion_2 _charm_2 _knowledge_2 _strength_2) (break `/Game/game/结构/Agent/Agent模拟属性` `_属性变更规则_2`))
  (`parent.执行交互`)
  (set `self.找到动作` false)
  (for _array_element (`self.自定义交互物结构`)
    (if (== (`.动作_7_2642A6D0444B5CFD19D0ABB180145703` (break `/Game/game/结构/Agent/自定义交互物结构` _array_element)) (`self.参数`))
      (set `self.找到动作` true)
      (`|ExecutionSequence`
        (:`then_0`
          (break))
        (:`then_1`
          (set `self.当前找到的动作` _array_element)
          (bind `_正在交互的agent_3` (`self.正在交互的Agent`)
            (:`then`
              (`/Game/game/AI/AI助手.服务器-在聊天框添加内容` `_正在交互的agent_3` (`KismetTextLibrary.Conv_StringToText` `_动作_2`))
              (`/Engine/EditorBlueprintResources/StandardMacros.IsValid` `_进入动画_2`
                (:`Is Valid`
                  (`/Game/game/AI/AI助手.服务器-交互效果设置` :`self` `_正在交互的agent_3` :`进入` true :`AnimMontage` `_进入动画_2` :`播放交互变换` `_交互位置_2` :`进入路径` (`self.交互样条线`))
                  (`/Engine/EditorBlueprintResources/StandardMacros.IsValid` `_持续动画_2`
                    (:`Is Valid`
                      (if (`/Game/game/AI/AI助手.正在播放动画` (`self.正在交互的Agent`)) :!label _label_2
                        (`KismetSystemLibrary.Delay` 0.01)
                        (goto _label_2)
                        (else
                          (`/Game/game/AI/AI助手.服务器-交互效果设置` :`self` (`self.正在交互的Agent`) :`进入` true :`AnimMontage` `_持续动画_2` :`播放交互变换` `_交互位置_3` :`进入路径` (`self.交互样条线`))
                          ;[1 1 1] 持续动画完成
                          (`KismetSystemLibrary.Delay` 20.0)
                          (`/Game/game/AI/AI助手.服务器-修改Agent属性` `_正在交互的agent_2` (`KismetTextLibrary.Conv_StringToText` `_动作`) _money _reputation _creativity _emotion _charm _knowledge _strength)
                          (`/Game/game/AI/AI助手.当前节点完成` `_正在交互的agent_2` true 0))))
                    (:`Is Not Valid`
                      ;[1 1 1] 进入动画完成
                      (if (`/Game/game/AI/AI助手.正在播放动画` (`self.正在交互的Agent`)) :!label _label_3
                        (`KismetSystemLibrary.Delay` 0.2)
                        (goto _label_3)
                        (else
                          (`/Game/game/AI/AI助手.服务器-修改Agent属性` `_正在交互的agent` (`KismetTextLibrary.Conv_StringToText` `_动作_4`) _money_2 _reputation_2 _creativity_2 _emotion_2 _charm_2 _knowledge_2 _strength_2)
                          (`/Game/game/AI/AI助手.当前节点完成` `_正在交互的agent` true 0))))))
                (:`Is Not Valid`
                  (`/Engine/EditorBlueprintResources/StandardMacros.IsValid` `_离开动画_2`
                    (:`Is Valid`
                      (`/Game/game/AI/AI助手.服务器-交互效果设置` :`self` (`self.正在交互的Agent`) :`进入` true :`AnimMontage` `_离开动画_2` :`播放交互变换` `_交互位置_3` :`进入路径` (`self.交互样条线`))
                      ;[1 1 1] 离开动画完成
                      (if (`/Game/game/AI/AI助手.正在播放动画` (`self.正在交互的Agent`)) :!label _label_4
                        (`KismetSystemLibrary.Delay` 0.2)
                        (goto _label_4)
                        (else
                          (`/Game/game/AI/AI助手.当前节点完成` (`self.正在交互的Agent`) true 0)
                          (bind `_正在交互的agent_4` (`self.正在交互的Agent`)
                            (:`then`
                              (`self.结束交互`)
                              (set `/Game/game/AI/AI助手.Agent正在可交互的物体` null `_正在交互的agent_4`))
                            (:`else`)))))
                    (:`Is Not Valid`
                      ;[1 1 1] 动画无效完成
                      (`/Game/game/AI/AI助手.当前节点完成` (`self.正在交互的Agent`) true 0))))))
            (:`else`
              (`/Game/game/AI/AI助手.当前节点完成` (`self.正在交互的Agent`) true 0)))))))
  ;[1 1 1] 未找到动作完成
  (if (not (`self.找到动作`))
    (`/Game/game/AI/AI助手.当前节点完成` (`self.正在交互的Agent`) true 0)))

(fn `UserConstructionScript`
  (`parent.UserConstructionScript`))