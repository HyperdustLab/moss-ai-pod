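; Meditation spot (打坐), an interactable object that AI Agents use to meditate.
; On a "Meditate" interaction, it sends the Agent along a spline into an idle montage at an arrow transform and applies attribute changes parsed from GameInstance JSON.
; It posts chat text, switches to an automatic camera after a delay, then completes the Agent's current node.
; Ending the interaction plays an exit montage at a second arrow and posts a stand-up message.
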(event `self.执行交互`
  (bind _returnvalue (`SceneComponent.K2_GetComponentToWorld` (`self.Arrow`)))
  (bind (_success `_钱` `_创造力` `_情绪` `_魅力` `_知识` `_力量` `_声望`) (`|Json` (`|GetArrayItem` (`/Game/game/INS.Agent属性变化` (cast `/Game/game/INS` (`GameplayStatics.GetGameInstance`) :!pure true)) 6)))
  (`parent.执行交互`)
  (if (== (`self.参数`) "Meditate")
    (bind `_正在交互的agent` (`self.正在交互的Agent`)
      (:`then`
        (`/Game/game/AI/AI助手.服务器-交互效果设置` `_正在交互的agent` true false "/Game/game/Resource_Pack/动画/打坐动画/Animations/retargeted/待机动画.待机动画" _returnvalue _returnvalue (`self.交互样条线`))
        (`/Game/game/AI/AI助手.服务器-修改Agent属性` (`self.正在交互的Agent`) "冥想" (`KismetStringLibrary.Conv_StringToInt` `_钱`) (`KismetStringLibrary.Conv_StringToInt` `_创造力`) (`KismetStringLibrary.Conv_StringToInt` `_情绪`) (`KismetStringLibrary.Conv_StringToInt` `_魅力`) (`KismetStringLibrary.Conv_StringToInt` `_知识`) (`KismetStringLibrary.Conv_StringToInt` `_力量`) (`KismetStringLibrary.Conv_StringToInt` `_声望`))
        (`/Game/game/AI/AI助手.服务器-在聊天框添加内容` (`self.正在交互的Agent`) "冥想")
        (`KismetSystemLibrary.Delay` 4.0)
        (`/Game/game/AI/AI助手.服务器-交互镜头` (`self.正在交互的Agent`) "NewEnumerator2" (`|MakeArray` (`self.镜头箭头组件1`) (`self.镜头箭头组件2`) (`self.镜头箭头组件3`)) self (0.0 0.0 45.0) true)
        (`KismetSystemLibrary.Delay` 20.0)
        (`/Game/game/AI/AI助手.当前节点完成` (`self.正在交互的Agent`) true 0))
      (:`else`))
    (else
      (`/Game/game/AI/AI助手.当前节点完成` (`self.正在交互的Agent`) true 0))))

(event `self.结束交互`
  (bind `_正在交互的agent` (`self.正在交互的Agent`))
  (bind _returnvalue (`SceneComponent.K2_GetComponentToWorld` (`self.Arrow1`)))
  (`parent.结束交互`)
  (`/Game/game/AI/AI助手.服务器-交互效果设置` `_正在交互的agent` false false "/Game/game/Resource_Pack/动画/休息动画_2/Animations/Sleep/StartEnd/下床.下床" _returnvalue _returnvalue (`self.交互样条线`))
  (`/Game/game/AI/AI助手.服务器-在聊天框添加内容` `_正在交互的agent` "站起"))

(fn `UserConstructionScript`
  (`parent.UserConstructionScript`))