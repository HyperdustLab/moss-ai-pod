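; Sports field (操场) Agent interactable offering Warm Up and Running activities, selected by the interaction parameter.
; Warm Up chains random montages through a Gate loop for 60 seconds before completing the Agent's node.
; Running raises move speed and sends the Agent twice along the spline's points, completing when movement finishes.
; Both post chat text and apply GameInstance JSON attribute changes; ending interaction restores walk speed.
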(event `self.执行交互`
  (bind `_正在交互的agent` (`self.正在交互的Agent`))
  (bind `_交互样条线` (`self.交互样条线`))
  (bind _newvar_1 (`self.NewVar_1`))
  (bind `_正在交互的agent_2` (`self.正在交互的Agent`))
  (bind `_参数` (`self.参数`))
  (bind _anim_montage (`self.Anim Montage`))
  (bind `_正在交互的agent_3` (`self.正在交互的Agent`))
  (bind (_success `_钱` `_创造力` `_情绪` `_魅力` `_知识` `_力量` `_声望`) (`|Json` (`|GetArrayItem` (`/Game/game/INS.Agent属性变化` (cast `/Game/game/INS` (`GameplayStatics.GetGameInstance`) :!pure true)) 7)))
  (bind (_success_2 `_钱_2` `_创造力_2` `_情绪_2` `_魅力_2` `_知识_2` `_力量_2` `_声望_2`) (`|Json` (`|GetArrayItem` (`/Game/game/INS.Agent属性变化` (cast `/Game/game/INS` (`GameplayStatics.GetGameInstance`) :!pure true)) 8)))
  (`parent.执行交互`)
  (if (== `_参数` "Warm Up")
    (`|ExecutionSequence`
      (:`then_0`
        (goto _label :!via `Open`))
      (:`then_1`
        (`/Engine/EditorBlueprintResources/StandardMacros.Gate` true :!label _label
          (:`Exit`
            (set `self.NewVar_1` (`|GetArrayItem` _anim_montage (`KismetMathLibrary.RandomIntegerInRange` 0 (- (`KismetArrayLibrary.Array_Length` _anim_montage) 1))))
            (`/Game/game/AI/AI助手.组播-播放动画蒙太奇` :`self` `_正在交互的agent_2` :`动画` _newvar_1 :`播放变换` (`self.GetTransform` `_正在交互的agent_2`))
            (`KismetSystemLibrary.Delay` (`AnimationAsset.GetPlayLength` _newvar_1))
            (goto _label))))
      (:`then_2`
        (`/Game/game/AI/AI助手.服务器-在聊天框添加内容` (`self.正在交互的Agent`) "热身锻炼")
        (`/Game/game/AI/AI助手.服务器-修改Agent属性` (`self.正在交互的Agent`) "热身" (`KismetStringLibrary.Conv_StringToInt` `_钱`) (`KismetStringLibrary.Conv_StringToInt` `_创造力`) (`KismetStringLibrary.Conv_StringToInt` `_情绪`) (`KismetStringLibrary.Conv_StringToInt` `_魅力`) (`KismetStringLibrary.Conv_StringToInt` `_知识`) (`KismetStringLibrary.Conv_StringToInt` `_力量`) (`KismetStringLibrary.Conv_StringToInt` `_声望`))
        (`KismetSystemLibrary.Delay` 60.0)
        (`/Game/game/AI/AI助手.当前节点完成` (`self.正在交互的Agent`) true 0)
        (goto _label :!via `Close`)))
    (elif (== `_参数` "Running")
      (`/Game/game/AI/AI助手.组播-播放动画蒙太奇` :`self` `_正在交互的agent`)
      (`/Game/game/AI/AI助手.服务器-在聊天框添加内容` `_正在交互的agent` "跑步")
      (`/Game/game/AI/AI助手.服务器-设置移动速度` `_正在交互的agent` 600.0)
      (`/Game/game/AI/AI助手.服务器-修改Agent属性` (`self.正在交互的Agent`) "跑步" (`KismetStringLibrary.Conv_StringToInt` `_钱_2`) (`KismetStringLibrary.Conv_StringToInt` `_创造力_2`) (`KismetStringLibrary.Conv_StringToInt` `_情绪_2`) (`KismetStringLibrary.Conv_StringToInt` `_魅力_2`) (`KismetStringLibrary.Conv_StringToInt` `_知识_2`) (`KismetStringLibrary.Conv_StringToInt` `_力量_2`) (`KismetStringLibrary.Conv_StringToInt` `_声望_2`))
      (for _index (range (`SplineComponent.GetNumberOfSplinePoints` `_交互样条线`))
        (`KismetArrayLibrary.Array_Add` (`self.跑道路径`) (`SplineComponent.GetLocationAtSplinePoint` `_交互样条线` _index "World")))
      (set `self.跑道额外路径` (`self.跑道路径`))
      (`KismetArrayLibrary.Array_Append` (`self.跑道路径`) (`self.跑道额外路径`))
      (add `/Game/game/AI/AI助手.移动完成分发器` `_正在交互的agent_3` (delegate `移动完成`))
      (`/Game/game/AI/AI助手.服务器-按路径移动` `_正在交互的agent_3` (`self.跑道路径`))
      (`KismetSystemLibrary.Delay` 0.2)
      (`KismetArrayLibrary.Array_Clear` (`self.跑道路径`))
      (`KismetArrayLibrary.Array_Clear` (`self.跑道额外路径`))
      (else
        (`/Game/game/AI/AI助手.当前节点完成` (`self.正在交互的Agent`) true 0)))))

(event `移动完成`
  (params (`成功` :type Boolean))
  (bind `_正在交互的agent` (`self.正在交互的Agent`))
  (remove `/Game/game/AI/AI助手.移动完成分发器` `_正在交互的agent` (delegate `移动完成`))
  (`/Game/game/AI/AI助手.当前节点完成` `_正在交互的agent` `成功` 0))

(event `self.结束交互`
  (bind `_正在交互的agent` (`self.正在交互的Agent`))
  (bind `_参数` (`self.参数`))
  (`parent.结束交互`)
  (`/Game/game/AI/AI助手.服务器-设置移动速度` `_正在交互的agent` (`/Game/game/AI/AI助手.默认行走速度` `_正在交互的agent`))
  (`self.结束交互完成清除变量`)
  (if (== `_参数` "Warm Up")
    (`/Game/game/AI/AI助手.组播-播放动画蒙太奇` :`self` (`self.正在交互的Agent`) :`停止` true)
    (elif (== `_参数` "Running")
      _)))

(fn `UserConstructionScript`
  (`parent.UserConstructionScript`))