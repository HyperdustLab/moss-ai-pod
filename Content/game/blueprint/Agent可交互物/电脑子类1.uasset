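; A computer subclass of an agent-interactable object that changes its screen visuals around an interaction.
; It extends two parent events, add screen animation (添加屏幕动画) and end interaction (结束交互), calling the parent logic first.
; The former sets slot 0 on SMTable01 and SMTable02 to the horizontal dynamic screen material, and the latter sets it to M_Screen_Dynamic1_Inst.
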(event `self.添加屏幕动画`
  (`parent.添加屏幕动画`)
  (`PrimitiveComponent.SetMaterial` (`self.SM_Table_01`) 0 "/Game/game/Resource_Pack/环境/SciFi_Server_Facility/Materials/MI_Screen_Dynamic_Horizontal.MI_Screen_Dynamic_Horizontal")
  (`PrimitiveComponent.SetMaterial` (`self.SM_Table_02`) 0 "/Game/game/Resource_Pack/环境/SciFi_Server_Facility/Materials/MI_Screen_Dynamic_Horizontal.MI_Screen_Dynamic_Horizontal"))

(event `/Game/game/blueprint/Agent可交互物/Agent可交互物父类.结束交互`
  (`parent.结束交互`)
  (`PrimitiveComponent.SetMaterial` (`self.SM_Table_01`) 0 "/Game/game/Resource_Pack/环境/SciFi_Server_Facility/Materials/Master_Materials/M_Screen_Dynamic1_Inst.M_Screen_Dynamic1_Inst")
  (`PrimitiveComponent.SetMaterial` (`self.SM_Table_02`) 0 "/Game/game/Resource_Pack/环境/SciFi_Server_Facility/Materials/Master_Materials/M_Screen_Dynamic1_Inst.M_Screen_Dynamic1_Inst"))

(fn `UserConstructionScript`
  (`parent.UserConstructionScript`))