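; Base Blueprint for objects that AI Agents can interact with, with empty execute and end events, presumably for child classes.
; The pre-interaction event locks the object to one Agent, reporting failure to others trying to enter, and routes enter or exit accordingly.
; A cleanup event releases the Agent and parameter.
; A sphere-trace helper detects other nearby pawns; nearest-location lookup logic is left disconnected.
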(event `服务器-设置所在位置`
  ;[1 1 1] 手动填写
)

(event `self.ReceiveBeginPlay`)

(event `交互前置`
  (params (Agent :type "/Game/game/AI/AI助手 Object Reference") (`参数` :type String) (`进入` :type Boolean))
  (if `进入`
    (bind `_正在交互的agent` (`self.正在交互的Agent`)
      (:`then`
        (if (== `_正在交互的agent` Agent)
          (set `self.正在交互的Agent` Agent :!label _label)
          (set `self.参数` `参数`)
          (`self.执行交互`)
          (else
            (`/Game/game/AI/AI助手.当前节点完成` Agent false 0))))
      (:`else`
        (goto _label)))
    (else
      (bind `_正在交互的agent_2` (`self.正在交互的Agent`)
        (:`then`
          (if (== `_正在交互的agent_2` Agent)
            (`self.结束交互`)
            (else
              (set `/Game/game/AI/AI助手.Agent正在可交互的物体` null Agent :!label _label_2))))
        (:`else`
          (goto _label_2))))))

(event `执行交互`)

(event `结束交互`)

(event `结束交互完成清除变量`
  (bind `_正在交互的agent` (`self.正在交互的Agent`)
    (:`then`
      (set `/Game/game/AI/AI助手.Agent正在可交互的物体` null `_正在交互的agent`))
    (:`else`
      _))
  (set `self.参数` "")
  (set `self.正在交互的Agent` null))

(fn `UserConstructionScript`)

(fn `存在其他玩家交互`
  (params (`排除的角色` :type "Actor Object Reference"))
  (returns (ReturnValue :type Boolean))
  (bind _returnvalue (`self.K2_GetActorLocation`))
  (bind (_outhit _returnvalue_2) (`KismetSystemLibrary.SphereTraceSingleForObjects` _returnvalue _returnvalue 100.0 (`|MakeArray` "ObjectTypeQuery3" :!type "EObjectTypeQuery Enum") false (`|MakeArray` `排除的角色`) "ForDuration"))
  (return _returnvalue_2))