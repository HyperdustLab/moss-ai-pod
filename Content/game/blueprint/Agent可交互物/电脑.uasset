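; Interactable computer that AI Agents sit at to carry out a work task passed as a colon-separated parameter string.
; Interaction plays a typing montage, posts to chat, removes the matching task from the Agent's work list and saves it.
; A looping timer waits until the Agent is near, then after a delay launches the GameInstance browser and applies configured attribute changes.
; Empty parameters fail the node; ending interaction plays stand-up.
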(event `添加屏幕动画`)

(event `self.执行交互`
  (bind `_参数` (`self.参数`))
  (bind `_正在交互的agent` (`self.正在交互的Agent`))
  (bind (_lefts _rights _returnvalue) (`KismetStringLibrary.Split` `_参数` ":"))
  (bind `_工作结构` (`/Game/game/AI/AI助手.工作结构` `_正在交互的agent`))
  (`parent.执行交互`)
  (set `self.启动浏览器` false)
  (bind `_正在交互的agent_2` (`self.正在交互的Agent`)
    (:`then`
      (if (`KismetStringLibrary.IsEmpty` `_参数`)
        ;[1 1 1] 窗口化
        (`/Game/game/AI/AI助手.当前节点完成` `_正在交互的agent_2` false 0)
        (else
          (if _returnvalue
            (set `self.启动浏览器` true))
          (`|ExecutionSequence`
            (:`then_0`
              (set `self.浏览器任务` _rights)
              (`/Game/game/AI/AI助手.服务器-交互效果设置` :`self` `_正在交互的agent_2` :`进入` true :`固定播放` true :`AnimMontage` "/Game/game/Resource_Pack/动画/办公动画/Animation/Root_Motion/键盘动画蒙太奇.键盘动画蒙太奇" :`播放交互变换` (`/Game/game/函数库.变换+变换` (`SceneComponent.K2_GetComponentToWorld` (`self.Arrow`)) (`KismetMathLibrary.Conv_VectorToTransform` (`/Game/game/AI/AI助手.坐姿偏移` `_正在交互的agent_2`))) :`进入路径` (`self.交互样条线`))
              (`/Game/game/AI/AI助手.服务器-在聊天框添加内容` (`self.正在交互的Agent`) (`KismetTextLibrary.Conv_StringToText` (`self.参数`)))
              (bind _returnvalue_2 (`KismetSystemLibrary.K2_SetTimerDelegate` (delegate `交互判断`) 1.0 true))
              (set `self.交互判断定时器柄` _returnvalue_2))
            (:`then_1`
              (for (_array_element _array_index) `_工作结构`
                (if (== (`.索引_9_F75E94CB4EFA0030B1D104B37E106E82` (break `/Game/game/结构/Agent/工作安排结构` _array_element)) (`KismetStringLibrary.Conv_StringToInt` (`.RightS` (`KismetStringLibrary.Split` _lefts "Task"))))
                  (`KismetArrayLibrary.Array_AddUnique` (`/Game/game/AI/AI助手.已完成的任务` (`self.正在交互的Agent`)) (`self.参数`))
                  (`KismetArrayLibrary.Array_Remove` `_工作结构` _array_index)))
              (`/Game/game/AI/AI助手.保存Agent扩展字段` `_正在交互的agent`))))))
    (:`else`)))

(event `交互判断`
  (bind _asins (cast `/Game/game/INS` (`GameplayStatics.GetGameInstance`) :!pure true))
  (bind (_success `_钱` `_创造力` `_情绪` `_魅力` `_知识` `_力量` `_声望`) (`|Json` (`|GetArrayItem` (`.String Array` (`|JsonToArray` (`/Game/game/INS.Agent工作配置` _asins))))))
  (bind `_正在交互的agent` (`self.正在交互的Agent`)
    (:`then`
      (if (not (> (`KismetMathLibrary.VSize` (- (`self.K2_GetActorLocation` `_正在交互的agent`) (`self.K2_GetActorLocation`))) 1000.0))
        (`KismetSystemLibrary.K2_ClearAndInvalidateTimerHandle` (`self.交互判断定时器柄`))
        (`self.添加屏幕动画`)
        (`KismetSystemLibrary.Delay` 5.0)
        (if (`self.启动浏览器`)
          (`/Game/game/INS.启动浏览器` _asins (`KismetTextLibrary.Conv_StringToText` (`self.浏览器任务`)))
          (`/Game/game/AI/AI助手.服务器-修改Agent属性` (`self.正在交互的Agent`) "使用电脑" (`KismetStringLibrary.Conv_StringToInt` `_钱`) (`KismetStringLibrary.Conv_StringToInt` `_创造力`) (`KismetStringLibrary.Conv_StringToInt` `_情绪`) (`KismetStringLibrary.Conv_StringToInt` `_魅力`) (`KismetStringLibrary.Conv_StringToInt` `_知识`) (`KismetStringLibrary.Conv_StringToInt` `_力量`) (`KismetStringLibrary.Conv_StringToInt` `_声望`))
          (else
            (`/Game/game/AI/AI助手.当前节点完成` (`self.正在交互的Agent`) true 0)))))
    (:`else`)))

(event `self.结束交互`
  (bind `_正在交互的agent` (`self.正在交互的Agent`))
  (`parent.结束交互`)
  (`/Game/game/AI/AI助手.服务器-交互效果设置` :`self` `_正在交互的agent` :`AnimMontage` "/Game/game/Resource_Pack/动画/休息动画_2/Animations/Sit/Default/StartEnd/左起立蒙太奇.左起立蒙太奇" :`播放交互变换` (`SceneComponent.K2_GetComponentToWorld` (`self.Arrow`)) :`进入路径` (`self.交互样条线`))
  (`/Game/game/AI/AI助手.服务器-在聊天框添加内容` `_正在交互的agent` "结束任务")
  (`KismetSystemLibrary.K2_ClearAndInvalidateTimerHandle` (`self.交互判断定时器柄`)))

(fn `UserConstructionScript`
  (`parent.UserConstructionScript`))