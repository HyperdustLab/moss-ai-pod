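; Library chair interactable that lets an Agent sit down, stand up or read.
; 执行交互 branches on the 参数 string, sending the Agent server calls for montage, transform, spline path and chat text, then reporting node completion, after fixed Delays for those three actions.
; Sitting also triggers an auto camera on the chair, while reading applies attribute changes from the INS GameInstance.
; 结束交互 plays the stand-up exit.
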(event `self.执行交互`
  (bind `_参数` (`self.参数`))
  (bind `_正在交互的agent` (`self.正在交互的Agent`))
  (bind `_交互样条线` (`self.交互样条线`))
  (bind _returnvalue (`SceneComponent.K2_GetComponentToWorld` (`self.Arrow`)))
  (bind (_success `_钱` `_创造力` `_情绪` `_魅力` `_知识` `_力量` `_声望`) (`|Json` (`|GetArrayItem` (`/Game/game/INS.Agent属性变化` (cast `/Game/game/INS` (`GameplayStatics.GetGameInstance`) :!pure true)) 5)))
  (`parent.执行交互`)
  (if (== `_参数` "Sit Down")
    (bind `_正在交互的agent_2` (`self.正在交互的Agent`)
      (:`then`
        (`/Game/game/AI/AI助手.服务器-交互效果设置` :`self` `_正在交互的agent_2` :`进入` true :`AnimMontage` "/Game/game/Resource_Pack/动画/休息动画_2/Animations/Sit/Default/StartEnd/正常坐下蒙太奇.正常坐下蒙太奇" :`播放交互变换` (`/Game/game/函数库.变换+变换` _returnvalue (`KismetMathLibrary.Conv_VectorToTransform` (`/Game/game/AI/AI助手.坐姿偏移` `_正在交互的agent_2`))) :`进入路径` `_交互样条线`)
        (`/Game/game/AI/AI助手.服务器-在聊天框添加内容` (`self.正在交互的Agent`) "坐下")
        (`KismetSystemLibrary.Delay` 4.0)
        (`/Game/game/AI/AI助手.服务器-交互镜头` (`self.正在交互的Agent`) "NewEnumerator2" (`|MakeArray` (`self.镜头箭头组件1`) (`self.镜头箭头组件2`) (`self.镜头箭头组件3`) (`self.镜头箭头组件4`)) self (0.0 0.0 40.0) true)
        (`KismetSystemLibrary.Delay` 10.0)
        (`/Game/game/AI/AI助手.当前节点完成` (`self.正在交互的Agent`) true 0 :!label _label))
      (:`else`))
    (elif (== `_参数` "Stand Up")
      (bind `_正在交互的agent_3` (`self.正在交互的Agent`)
        (:`then`
          (`/Game/game/AI/AI助手.服务器-交互效果设置` :`self` `_正在交互的agent_3` :`AnimMontage` "/Game/game/Resource_Pack/动画/休息动画_2/Animations/Sit/Default/StartEnd/左起立蒙太奇.左起立蒙太奇" :`播放交互变换` _returnvalue :`进入路径` `_交互样条线`)
          (`/Game/game/AI/AI助手.服务器-在聊天框添加内容` (`self.正在交互的Agent`) "站起")
          (`KismetSystemLibrary.Delay` 4.0)
          (goto _label))
        (:`else`))
      (elif (== `_参数` "Read")
        (bind `_正在交互的agent_4` (`self.正在交互的Agent`)
          (:`then`
            (`/Game/game/AI/AI助手.服务器-交互效果设置` :`self` `_正在交互的agent_4` :`进入` true :`AnimMontage` "/Game/game/Resource_Pack/动画/办公动画/Animation/Root_Motion/签署文件蒙太奇.签署文件蒙太奇" :`播放交互变换` (`/Game/game/函数库.变换+变换` (`SceneComponent.K2_GetComponentToWorld` (`self.Arrow1`)) (`KismetMathLibrary.Conv_VectorToTransform` (`/Game/game/AI/AI助手.坐姿偏移` `_正在交互的agent_4`))) :`进入路径` (`self.交互样条线`))
            (`/Game/game/AI/AI助手.服务器-在聊天框添加内容` `_正在交互的agent` "阅读")
            (`/Game/game/AI/AI助手.服务器-修改Agent属性` `_正在交互的agent` "阅读" (`KismetStringLibrary.Conv_StringToInt` `_钱`) (`KismetStringLibrary.Conv_StringToInt` `_创造力`) (`KismetStringLibrary.Conv_StringToInt` `_情绪`) (`KismetStringLibrary.Conv_StringToInt` `_魅力`) (`KismetStringLibrary.Conv_StringToInt` `_知识`) (`KismetStringLibrary.Conv_StringToInt` `_力量`) (`KismetStringLibrary.Conv_StringToInt` `_声望`))
            (`KismetSystemLibrary.Delay` 20.0)
            (goto _label))
          (:`else`))
        (else
          (`/Game/game/AI/AI助手.当前节点完成` (`self.正在交互的Agent`) true 0))))))

(event `self.结束交互`
  (bind `_正在交互的agent` (`self.正在交互的Agent`))
  (`parent.结束交互`)
  (`/Game/game/AI/AI助手.服务器-交互效果设置` :`self` `_正在交互的agent` :`AnimMontage` "/Game/game/Resource_Pack/动画/休息动画_2/Animations/Sit/Default/StartEnd/左起立蒙太奇.左起立蒙太奇" :`播放交互变换` (`SceneComponent.K2_GetComponentToWorld` (`self.Arrow`)) :`进入路径` (`self.交互样条线`))
  (`/Game/game/AI/AI助手.服务器-在聊天框添加内容` `_正在交互的agent` "站起"))

(fn `UserConstructionScript`
  (`parent.UserConstructionScript`))