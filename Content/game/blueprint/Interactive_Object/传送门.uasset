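; Teleporter actor (传送门) that sends a player entering its sphere to a linked partner portal (对应传送门).
; On authority, if the player has no interactable item and the portal is not cooling down, it spawns a sigil effect with sound, waits briefly, then calls the player's teleport to the partner's 传送位置.
; Both portals share the cooldown flag during the delay, clearing it right after teleporting.
; The construction script sets the Text3D label from 内容.
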(event `self.ReceiveBeginPlay`
  (`parent.ReceiveBeginPlay`))

(event `生成特效和声音`
  (bind (_returnvalue_location _returnvalue_rotation) (`KismetMathLibrary.BreakTransform` (`SceneComponent.K2_GetComponentToWorld` (`self.特效和音效位置`))))
  (bind _returnvalue (`GameplayStatics.SpawnEmitterAtLocation` "/Game/ZY/fx/SigilVFXMaterialPack/VFX/Sigils/P_Sigil_20.P_Sigil_20" _returnvalue_location _returnvalue_rotation (3.0 3.0 3.0)))
  (`GameplayStatics.SpawnSoundAttached` "/Game/lhy/music/音效/太空飞船控制反应.太空飞船控制反应" _returnvalue "None" _returnvalue_location _returnvalue_rotation "KeepWorldPosition" true 1.0 1.0 0.0 null null))

(event `self.ReceiveTick`
  (params (DeltaSeconds :type "Float (single-precision)"))
  (`parent.ReceiveTick` DeltaSeconds))

(event `self.Sphere_0.OnComponentBeginOverlap`
  (params (OverlappedComponent :type "PrimitiveComponent Object Reference") (OtherActor :type "Actor Object Reference") (OtherComp :type "PrimitiveComponent Object Reference") (OtherBodyIndex :type Integer) (bFromSweep :type Boolean) (SweepResult :type "HitResult Structure (by ref)"))
  (bind `_as玩家_0` (`self.As玩家_0`))
  (bind `_as玩家` (cast `/Game/game/玩家` OtherActor))
  (switch `/Game/game/枚举/可交互物体枚举` (`/Game/game/玩家.正在交互的枚举` `_as玩家`)
    (:`NewEnumerator0`
      (set `self.As玩家_0` `_as玩家`)
      (`/Engine/EditorBlueprintResources/ActorMacros.Switch Has Authority`
        (:`Authority`
          (if (not (`self.正在冷却`))
            (bind `_对应传送门` (`self.对应传送门`)
              (:`then`
                (set `self.正在冷却` true)
                (set `/Game/game/blueprint/Interactive_Object/传送门.正在冷却` true `_对应传送门`)
                (`self.生成特效和声音`)
                (`KismetSystemLibrary.Delay` 1.5)
                (bind `_传送位置` (`/Game/game/blueprint/Interactive_Object/传送门.传送位置` `_对应传送门`))
                (`/Game/game/玩家.传送自身` `_as玩家_0` (`SceneComponent.K2_GetComponentLocation` `_传送位置`) (`SceneComponent.K2_GetComponentRotation` `_传送位置`) (`Pawn.GetController` `_as玩家_0`) false)
                (set `self.正在冷却` false)
                (set `/Game/game/blueprint/Interactive_Object/传送门.正在冷却` false `_对应传送门`))
              (:`else`))))))))

(fn `UserConstructionScript`
  (`parent.UserConstructionScript`)
  (`Text3DComponent.SetText` (`self.Text3D`) (`self.内容`)))