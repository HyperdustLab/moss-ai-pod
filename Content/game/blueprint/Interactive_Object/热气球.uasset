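; Rideable multiplayer hot air balloon interactive object with a seat limit, a driver chosen by owner ID or first seat, and a client-spawned camera boom.
; Server Tick moves it from rise and camera-yaw-relative steering input, using box traces for ground detection and sinking it when empty.
; Clients interpolate toward the server position.
; A dynamic material shows a downloaded URL image or random pattern on non-scene balloons.
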(event `self.进行交互`
  (params (`是否进入` :type Boolean) (`玩家` :type "/Game/game/玩家 Object Reference") (Agent :type "/Game/game/AI/AI助手 Object Reference"))
  (bind `_所有交互的玩家` (`self.所有交互的玩家`))
  (bind `_当前交互的玩家` (`self.当前交互的玩家`))
  (bind _returnvalue (== `玩家` (`Controller.K2_GetPawn` (`GameplayStatics.GetPlayerController` 0))))
  (`parent.进行交互` `是否进入` `玩家` null)
  (if `是否进入`
    (if (> (+ (`self.已交互人数`) 1) (`self.可交互上限`))
      ;[1 1 1] 人数上限提示
      (`/Engine/EditorBlueprintResources/ActorMacros.Switch Has Authority`
        (:`Remote`
          (if (== (`Controller.K2_GetPawn` (`GameplayStatics.GetPlayerController` 0)) `玩家`)
            (`/Game/game/函数库.消息提示` "没有空余的位置"))))
      (else
        (`/Engine/EditorBlueprintResources/ActorMacros.Switch Has Authority`
          (:`Authority`
            (`KismetArrayLibrary.Array_AddUnique` `_所有交互的玩家` `_当前交互的玩家`)
            ;[1 1 1] 进入服务器
            (`self.服务器-设置所有玩家` `_所有交互的玩家`)
            (`self.服务器-设置乘坐位置`))
          (:`Remote`
            (if _returnvalue
              ;[1 1 1] 进入客户端
              (bind _returnvalue_2 (`|SpawnActorFromClass` "/Game/game/blueprint/Decoration/摄像机摇臂.摄像机摇臂_C" (`KismetMathLibrary.MakeTransform` (`KismetMathLibrary.MakeVector` (.x (`self.K2_GetActorLocation`)) (.y (`self.K2_GetActorLocation`)) (+ (.z (`self.K2_GetActorLocation`)) 2000.0))) "Undefined" "OverrideRootScale" null null null (2000.0 6000.0) 5000.0))
              (set `self.摄像机摇臂` _returnvalue_2)
              (`self.K2_AttachToActor` _returnvalue_2 self "None" "KeepWorld" "KeepWorld" "KeepWorld" true)
              (`KismetSystemLibrary.Delay` 0.5)
              (`/Game/game/玩家.设置摄像机摇臂` (`self.当前交互的玩家`) _returnvalue_2 true))))))
    (else
      (`/Engine/EditorBlueprintResources/ActorMacros.Switch Has Authority`
        (:`Authority`
          (`KismetArrayLibrary.Array_Remove` `_所有交互的玩家` (`KismetArrayLibrary.Array_Find` `_所有交互的玩家` `_当前交互的玩家`))
          ;[1 1 1] 离开服务器
          (`self.服务器-设置所有玩家` `_所有交互的玩家`)
          (`KismetSystemLibrary.Delay` 0.2)
          (`self.服务器-设置交互枚举` "NewEnumerator0")
          (`self.玩家交互的actor` null)
          (`self.进入` false))
        (:`Remote`
          (if _returnvalue
            ;[1 1 1] 离开客户端
            (`/Game/game/玩家.设置摄像机摇臂` `玩家` null false)
            (`self.结束交互`)
            (`self.K2_DestroyActor` (`self.摄像机摇臂`))))))))

(event `在服务器上运行`
  (set `self.图片链接` (`self.图片链接`)))

(event `设置热气球贴图`
  (`MaterialInstanceDynamic.SetTextureParameterValue` (`self.动态材质实例_0`) "贴图" (select `int` (`self.贴图索引`) :`0` null :`1` null :`2` null :`3` null :`4` null :`5` null :`6` null :`7` "/Game/game/图片/热气球图片/T_Pattern_06.T_Pattern_06" :`8` "/Game/game/图片/热气球图片/T_Pattern_06.T_Pattern_06" :!type "Texture Object Reference") :!label _label))

(event `self.ReceiveBeginPlay`
  (bind `_图片链接` (`self.图片链接`))
  (`parent.ReceiveBeginPlay`)
  (`|ExecutionSequence`
    (:`then_0`
      (`/Engine/EditorBlueprintResources/ActorMacros.Switch Has Authority`
        (:`Authority`
          (`self.在服务器上运行`))))
    (:`then_1`
      (`KismetSystemLibrary.Delay` 1.0)
      (cast `/Game/game/PLAY` (`GameplayStatics.GetPlayerController` 0) :!label _label_2
        (:`then`
          (if (`self.是否为场景物体`)
            _
            (elif (`KismetStringLibrary.IsEmpty` `_图片链接`)
              (`/Engine/EditorBlueprintResources/ActorMacros.Switch Has Authority`
                (:`Authority`
                  (`self.随机设置热气球贴图`))
                (:`Remote`
                  (goto _label)))
              (else
                (`KismetSystemLibrary.PrintText` (`KismetTextLibrary.Conv_StringToText` `_图片链接`) true true (struct :`R` 0.14885 :`B` 1.0 :`A` 1.0) 10.0)
                (bind _texture (`/Game/game/蓝图宏库.图片下载` `_图片链接`)
                  (:`On Success`
                    (`MaterialInstanceDynamic.SetTextureParameterValue` (`self.动态材质实例_0`) "贴图" _texture)))))))
        (:`CastFailed`
          (`KismetSystemLibrary.Delay` 1.0)
          (goto _label_2))))
    (:`then_2`
      (set `self.服务器上的位置` (`self.K2_GetActorLocation`))
      (set `self.是否启用tick` true))))

(event `随机设置热气球贴图`
  (set `self.贴图索引` (`KismetMathLibrary.RandomIntegerInRange` 0 8))
  (`self.设置热气球贴图`))

(event `服务器-设置服务器位置`
  (params (`服务器上的位置` :type "Vector Structure"))
  (set `self.服务器上的位置` `服务器上的位置`))

(event `服务器-前后输入`
  (params (`前后输入` :type "Float (double-precision)"))
  ;[1 1 1] 输入
  (set `self.前后输入` `前后输入`))

(event `前后`
  (params (`前后输入` :type "Float (double-precision)"))
  ;[1 1 1] 输入
  (`self.服务器-前后输入` `前后输入`))

(event `服务器-左右输入`
  (params (`左右输入` :type "Float (double-precision)"))
  ;[1 1 1] 输入
  (set `self.左右输入` `左右输入`))

(event `左右`
  (params (`左右输入` :type "Float (double-precision)"))
  ;[1 1 1] 输入
  (`self.服务器-左右输入` `左右输入`))

(event `上下`
  (params (`是否上升` :type Boolean))
  ;[1 1 1] 输入
  (set `self.是否上升` `是否上升`)
  (`SceneComponent.SetVisibility` (`self.SM_Flame`) (`self.是否上升`) false))

(event `服务器-是否上升`
  (params (`是否上升` :type Boolean))
  ;[1 1 1] 输入
  (set `self.是否上升` `是否上升`))

(event `视角旋转`
  (params (`摄像机旋转` :type "Rotator Structure"))
  ;[1 1 1] 输入
  (`self.服务器-旋转` `摄像机旋转`))

(event `服务器-旋转`
  (params (`摄像机旋转` :type "Rotator Structure"))
  ;[1 1 1] 输入
  (set `self.摄像机旋转` `摄像机旋转`))

(event `self.ReceiveTick`
  (params (DeltaSeconds :type "Float (single-precision)"))
  (bind (_returnvalue_x _returnvalue_y _returnvalue_z) (`KismetMathLibrary.BreakVector` (`self.K2_GetActorLocation`)))
  (bind _returnvalue (`self.K2_GetActorLocation`))
  (bind _returnvalue_2 (`self.K2_GetActorLocation`))
  (bind _returnvalue_3 (`self.K2_GetActorLocation`))
  (bind `_左右输入` (`self.左右输入`))
  (bind `_前后输入` (`self.前后输入`))
  (bind _yaw (.yaw (`self.摄像机旋转`)))
  (bind (_returnvalue_x_2 _returnvalue_y_2) (`KismetMathLibrary.BreakVector` (+ (* (`KismetMathLibrary.GetForwardVector` (`KismetMathLibrary.MakeRotator` 0.0 0.0 _yaw)) (* `_前后输入` 25.0)) (+ _returnvalue (* (`KismetMathLibrary.GetRightVector` (`KismetMathLibrary.MakeRotator` 0.0 0.0 _yaw)) (* `_左右输入` 25.0))))))
  ;[1 1 1] 移动
  (`parent.ReceiveTick` DeltaSeconds)
  (if (`self.是否启用tick`)
    (`/Engine/EditorBlueprintResources/ActorMacros.Switch Has Authority`
      (:`Authority`
        (if (> (`self.已交互人数`) 0)
          (`|ExecutionSequence`
            (:`then_0`
              (bind (_outhit _returnvalue_4) (`KismetSystemLibrary.BoxTraceSingle` _returnvalue_2 (`KismetMathLibrary.MakeVector` (.x _returnvalue_2) (.y _returnvalue_2) (- (.z _returnvalue_2) 5.0)) (80.0 80.0 0.0) (struct) "TraceTypeQuery1"))
              (if _returnvalue_4
                (bind _returnvalue_5 (select `bool` (`self.是否上升`) :`false` (select `bool` _returnvalue_4 :`false` -10.0) :`true` 14.0))
                (set `self.服务器上的位置` (`KismetMathLibrary.MakeVector` (.x (`self.K2_GetActorLocation`)) (.y (`self.K2_GetActorLocation`)) (+ (.z (`self.K2_GetActorLocation`)) _returnvalue_5)) :!label _label_3)
                (elif (or (!= `_左右输入` 0.0) (!= `_前后输入` 0.0))
                  (set `self.服务器上的位置` (`KismetMathLibrary.MakeVector` _returnvalue_x_2 _returnvalue_y_2 (+ (.z _returnvalue) _returnvalue_5)))
                  (else
                    (goto _label_3))))
              (`self.K2_SetActorLocation` (`self.服务器上的位置`)))
            (:`then_1`
              (goto _label_4 :!via `Reset`)))
          (else
            (`/Engine/EditorBlueprintResources/StandardMacros.DoOnce` false :!label _label_4
              (:`Completed`
                (bind (_outhit_2 _returnvalue_6) (`KismetSystemLibrary.BoxTraceSingle` _returnvalue_3 (`KismetMathLibrary.MakeVector` (.x _returnvalue_3) (.y _returnvalue_3) (- (.z _returnvalue_3) 5.0)) (100.0 100.0 0.0) (struct) "TraceTypeQuery1"))
                (if (not _returnvalue_6)
                  (cast `/Game/game/PLAY` (`GameplayStatics.GetPlayerController` 0)
                    (:`then`
                      (set `self.服务器上的位置` (`KismetMathLibrary.MakeVector` _returnvalue_x _returnvalue_y (+ _returnvalue_z -6.0)))
                      (`self.K2_SetActorLocation` (`self.服务器上的位置`))
                      (goto _label_4 :!via `Reset`))
                    (:`CastFailed`
                      (goto _label_4 :!via `Reset`)))))))))
      (:`Remote`
        (`self.K2_SetActorLocation` (`KismetMathLibrary.VInterpTo` (`self.K2_GetActorLocation`) (`self.服务器上的位置`) DeltaSeconds 100.0))))))

(event `进入`
  (params (`是否进入` :type Boolean))
  (bind `_拥有者id` (`self.拥有者ID`))
  (bind `_当前交互的玩家` (`self.当前交互的玩家`))
  (if `是否进入`
    (`|ExecutionSequence`
      (:`then_0`
        (`self.服务器-附加玩家` true)
        (`self.服务器-设置玩家变换` (`/Game/game/函数库.变换+变换` (`|GetArrayItem` (`self.交互进入偏移`) (- (`self.乘坐的位置`) 1)) (`self.GetTransform`)))
        (set `/Game/game/玩家.玩家是否在混合视图` true `_当前交互的玩家`))
      (:`then_1`
        (if (> (`KismetStringLibrary.Len` `_拥有者id`) 0)
          (if (`KismetStringLibrary.EqualEqual_StrStr` `_拥有者id` (`/Game/game/玩家.用户ID` `_当前交互的玩家`))
            (set `/Game/game/玩家.是否正在驾驶` true `_当前交互的玩家` :!label _label_5))
          (elif (== (`self.乘坐的位置`) 1)
            (goto _label_5)))))
    (else
      (set `/Game/game/玩家.是否正在驾驶` false `_当前交互的玩家`)
      (`self.服务器-附加玩家` false)
      (`self.服务器-设置玩家变换` (`KismetMathLibrary.MakeTransform` (+ (`self.K2_GetActorLocation` `_当前交互的玩家`) (* (`self.GetActorForwardVector` `_当前交互的玩家`) 200.0))))
      (set `/Game/game/玩家.玩家是否在混合视图` false `_当前交互的玩家`))))

(event `服务器-附加玩家`
  (params (`是否进入` :type Boolean))
  (`self.组播-附加玩家` `是否进入`))

(event `组播-附加玩家`
  (params (`是否进入` :type Boolean))
  (if `是否进入`
    (`/Game/game/蓝图宏库.将玩家附加到目标` (`self.当前交互的玩家`) self true true)
    (else
      (`/Game/game/蓝图宏库.将玩家附加到目标` (`self.当前交互的玩家`) self))))

(fn `UserConstructionScript`
  (bind _returnvalue (`PrimitiveComponent.CreateDynamicMaterialInstance` (`self.StaticMesh`) 1 "/Game/ZY/材质/材质实例/热气球材质_Inst.热气球材质_Inst" "None"))
  (set `self.动态材质实例_0` _returnvalue))