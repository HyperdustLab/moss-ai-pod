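; Scene live-stream actor (场景直播) that plays a video stream in the world through a media player and a media sound component added at BeginPlay.
; A callback reads the stream URL from a VaRest JSON response, then opens and plays it.
; The local pawn leaving the Box pauses playback.
; Entering does nothing: the overlap branch is empty, and the debounced GET request to the game instance's API is disconnected.
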(event `self.ReceiveBeginPlay`
  (`parent.ReceiveBeginPlay`)
  (`AddComponent|NODE_AddMediaSoundComponent-0`))

(event `self.Box.OnComponentBeginOverlap`
  (params (OverlappedComponent :type "PrimitiveComponent Object Reference") (OtherActor :type "Actor Object Reference") (OtherComp :type "PrimitiveComponent Object Reference") (OtherBodyIndex :type Integer) (bFromSweep :type Boolean) (SweepResult :type "HitResult Structure (by ref)"))
  (`/Engine/EditorBlueprintResources/ActorMacros.Switch Has Authority`
    (:`Remote`
      (if (== OtherActor (`Controller.K2_GetPawn` (`GameplayStatics.GetPlayerController` 0)))
        _))))

(event `获取场景视频链接`
  (params (Request :type "VaRestRequestJSON Object Reference"))
  (bind `_json视频` (`self.Json视频`))
  (bind `_媒体播放器` (`self.媒体播放器`))
  (bind `_流媒体源` (`self.流媒体源`))
  (bind _returnvalue (`VaRestJsonObject.GetStringField` `_json视频` "result"))
  (bind _returnvalue_2 (`VaRestRequestJSON.GetResponseContentAsString` Request false))
  (`VaRestJsonObject.DecodeJson` `_json视频` _returnvalue_2 false)
  (set `StreamMediaSource.StreamUrl` _returnvalue `_流媒体源`)
  (`MediaPlayer.OpenSource` `_媒体播放器` `_流媒体源`)
  (`MediaPlayer.Play` `_媒体播放器`)
  (`KismetSystemLibrary.PrintString` _returnvalue true true (struct :`G` 0.66 :`B` 1.0 :`A` 1.0) 5.0))

(event `self.Box.OnComponentEndOverlap`
  (params (OverlappedComponent :type "PrimitiveComponent Object Reference") (OtherActor :type "Actor Object Reference") (OtherComp :type "PrimitiveComponent Object Reference") (OtherBodyIndex :type Integer))
  (if (== OtherActor (`Controller.K2_GetPawn` (`GameplayStatics.GetPlayerController` 0)))
    (`MediaPlayer.Pause` (`self.媒体播放器`))))

(fn `UserConstructionScript`
  (`parent.UserConstructionScript`))