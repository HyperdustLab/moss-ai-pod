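; Procedural model actor (程序化模型) that builds a collidable mesh from a list of anchor positions.
; The Construction Script runs 生成锚点, which optionally adds small static mesh reference balls at the anchors, then calls 绘制模型.
; 绘制模型 uses the anchors as vertices and computes triangle-strip indices with alternating winding for the ProceduralMesh section.
; The loop count is one third of the point count plus three, so it does not fit every anchor count.
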(event `self.ReceiveBeginPlay`)

(event `生成锚点`
  (if (`self.生成参考球`)
    (for _array_element (`self.锚点位置`)
      (bind _returnvalue (`AddComponent|NODE_AddStaticMeshComponent-0` :`RelativeTransform` (`KismetMathLibrary.MakeTransform` _array_element (struct) (0.2 0.2 0.2))))
      (`KismetArrayLibrary.Array_Add` (`self.锚点`) _returnvalue)))
  (`self.绘制模型`))

(event `绘制模型`
  (bind `_当前三角面索引` (`self.当前三角面索引`))
  (set `self.顶点位置` (`self.锚点位置`))
  (for _index (range 1 (+ (+ (`.ReturnValue` (`KismetMathLibrary.FMod` (`KismetMathLibrary.Conv_IntToDouble` (`KismetArrayLibrary.Array_Length` (`self.顶点位置`))) 3.0)) 3) 1))
    (bind _returnvalue (+ (- _index 1) (- (* _index 3) (* (- _index 1) 3))))
    (bind _returnvalue_2 (== (`KismetMathLibrary.FMod` (`KismetMathLibrary.Conv_IntToDouble` _index) 2.0) 0.0))
    (`KismetArrayLibrary.Array_Add` `_当前三角面索引` (- _returnvalue (select `bool` _returnvalue_2 :`false` 3 :`true` 2)))
    (`KismetArrayLibrary.Array_Add` `_当前三角面索引` (- _returnvalue (select `bool` (not _returnvalue_2) :`false` 3 :`true` 2)))
    (`KismetArrayLibrary.Array_Add` `_当前三角面索引` (- _returnvalue 1)))
  (`ProceduralMeshComponent.CreateMeshSection_LinearColor` :`self` (`self.ProceduralMesh`) :`Vertices` (`self.顶点位置`) :`Triangles` (`self.当前三角面索引`) :`bCreateCollision` true))

(fn `UserConstructionScript`
  (`parent.UserConstructionScript`)
  (`self.生成锚点`))