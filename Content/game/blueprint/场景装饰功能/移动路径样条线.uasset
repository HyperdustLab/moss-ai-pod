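; Scene-decoration Blueprint that defines a movement path as a spline, built at runtime.
; On BeginPlay it clears the Spline component, then adds a point at the world location of each entry in the 位置 (positions) array, in array order.
; The construction script is empty, and nothing in this graph moves objects along the path.
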(event `self.ReceiveBeginPlay`
  (bind `_位置` (`self.位置`))
  (bind _spline (`self.Spline`))
  (`SplineComponent.ClearSplinePoints` _spline true)
  (for _index (range (`KismetArrayLibrary.Array_Length` `_位置`))
    (`SplineComponent.AddSplinePoint` _spline (`.WorldLocation` (break `CPathNode` (`|GetArrayItem` `_位置` _index))) "World" true)))

(fn `UserConstructionScript`)