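; Level streaming trigger actor (关卡卸载) that loads a named sublevel around the player and their AI assistant, and unloads it once both leave.
; Box overlap by either character passes a DoOnce to load the level without blocking and start a looping check timer.
; The timer compares both characters' distances against the box's larger horizontal extent plus a margin, then unloads the level, clears itself and resets the DoOnce.
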(event `self.Box.OnComponentBeginOverlap`
  (params (OverlappedComponent :type "PrimitiveComponent Object Reference") (OtherActor :type "Actor Object Reference") (OtherComp :type "PrimitiveComponent Object Reference") (OtherBodyIndex :type Integer) (bFromSweep :type Boolean) (SweepResult :type "HitResult Structure (by ref)"))
  (bind _asplay (cast `/Game/game/PLAY` (`GameplayStatics.GetPlayerController` 0) :!pure true))
  (bind `_as角色` (cast `Character` OtherActor))
  (if (== `_as角色` (`/Game/game/PLAY.玩家` _asplay))
    (`/Engine/EditorBlueprintResources/StandardMacros.DoOnce` false :!label _label
      (:`Completed`
        (set `self.角色` `_as角色`)
        (`GameplayStatics.LoadStreamLevel` (`self.关卡名称`) true)
        (bind _returnvalue (`KismetSystemLibrary.K2_SetTimerDelegate` (delegate `卸载定时器`) 2.0 true))
        (set `self.卸载定时器柄` _returnvalue)))
    (elif (== `_as角色` (`/Game/game/PLAY.Agent助手` _asplay))
      (goto _label))))

(event `卸载定时器`
  (bind _x (.x (`BoxComponent.GetScaledBoxExtent` (`self.Box`))))
  (bind _y (.y (`BoxComponent.GetScaledBoxExtent` (`self.Box`))))
  (bind _returnvalue (+ (select `bool` (> _x _y) :`false` _y :`true` _x) 4000.0))
  (bind `_角色` (`self.角色`)
    (:`then`
      (if (> (`KismetMathLibrary.VSize` (- (`self.K2_GetActorLocation` `_角色`) (`self.K2_GetActorLocation`))) _returnvalue)
        (bind `_asai助手` (cast `/Game/game/AI/AI助手` `_角色`)
          (:`then`
            (if (> (`KismetMathLibrary.VSize` (- (`self.K2_GetActorLocation` (`/Game/game/AI/AI助手.Agent拥有的玩家` `_asai助手`)) (`self.K2_GetActorLocation`))) _returnvalue)
              (`KismetSystemLibrary.K2_ClearAndInvalidateTimerHandle` (`self.卸载定时器柄`) :!label _label_2)
              (`GameplayStatics.UnloadStreamLevel` (`self.关卡名称`))
              (goto _label :!via `Reset`)))
          (:`CastFailed`
            (bind `_as玩家` (cast `/Game/game/玩家` `_角色`))
            (if (> (`KismetMathLibrary.VSize` (- (`self.K2_GetActorLocation` (`/Game/game/玩家.生成的AI助手` `_as玩家`)) (`self.K2_GetActorLocation`))) _returnvalue)
              (goto _label_2))))))
    (:`else`)))

(fn `UserConstructionScript`)