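; Placeable location marker actor for the Agent schedule system, hidden at runtime and labelled with its place name via a Text3D component.
; On BeginPlay it fills a list of random-position candidates from its own location plus the world locations of the Arrow component's child components.
; On the server it registers itself in the game mode's Agent coordinate list.
; The construction script refreshes the label so the name shows in the editor.
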(event `self.ReceiveBeginPlay`
  (`self.SetActorHiddenInGame` true)
  (`self.设置名称显示`)
  (`KismetArrayLibrary.Array_Add` (`self.坐标随机位置`) (`self.K2_GetActorLocation`))
  (for _array_element (`SceneComponent.GetChildrenComponents` (`self.Arrow`) false)
    (`KismetArrayLibrary.Array_Add` (`self.坐标随机位置`) (`SceneComponent.K2_GetComponentLocation` _array_element)))
  (`/Engine/EditorBlueprintResources/ActorMacros.Switch Has Authority`
    (:`Authority`
      (`KismetArrayLibrary.Array_Add` (`/Game/game/1GAME.Agent坐标` (cast `/Game/game/1GAME` (`GameplayStatics.GetGameMode`) :!pure true)) self))))

(event `设置名称显示`
  (set `Text3DComponent.Text` (`KismetTextLibrary.Conv_StringToText` (`self.地点名称`)) (`self.Text3D`)))

(fn `UserConstructionScript`
  (`self.设置名称显示`))