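; Roaming camera actor that slowly drifts while keeping a target actor in view.
; The focus event stores an arrow, offset and target, rolls a random drift vector, and starts a fast looping timer, or clears it when movement is off or the target is invalid.
; While the Agent's social state matches the first enum entry, each tick moves with sweep and smoothly rotates toward the offset target, clamping pitch and yaw around the arrow's rotation.
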(event `self.ReceiveBeginPlay`
  (`self.服务器-设置agent` (`self.agent`)))

(event `服务器-设置agent`
  (params (agent :type "/Game/game/AI/AI助手 Object Reference"))
  (set `self.agent` agent))

(event `聚焦物体`
  (params (`当前箭头` :type "ArrowComponent Object Reference") (`偏移量` :type "Vector Structure") (actor :type "Actor Object Reference") (`开启移动` :type Boolean))
  (set `self.当前箭头` `当前箭头`)
  (set `self.偏移量` `偏移量`)
  (set `self.聚集目标` actor)
  (if `开启移动`
    (`self.聚集目标`
      (:`then`
        (bind _returnvalue (`KismetSystemLibrary.K2_SetTimerDelegate` (delegate `自定义事件`) 0.01 true))
        (set `self.NewVar` _returnvalue)
        (set `self.随机移动` (+ (* (`self.GetActorRightVector`) (`KismetMathLibrary.RandomFloatInRange` -0.06 0.06)) (* (`self.GetActorUpVector`) (`KismetMathLibrary.RandomFloatInRange` -0.01 0.01)) (* (`self.GetActorForwardVector`) (`KismetMathLibrary.RandomFloatInRange` -0.1 0.003)))))
      (:`else`
        (`KismetSystemLibrary.K2_ClearAndInvalidateTimerHandle` (`self.NewVar`) :!label _label)))
    (else
      (goto _label))))

(event `自定义事件`
  (bind _pitch (.pitch (`SceneComponent.K2_GetComponentRotation` (`self.当前箭头`))))
  (bind _yaw (.yaw (`SceneComponent.K2_GetComponentRotation` (`self.当前箭头`))))
  (if (`|EnumEquality` (`/Game/game/AI/AI助手.agent社交状态` (`self.agent`)) "NewEnumerator0")
    (`self.K2_AddActorWorldOffset` (`self.随机移动`) true)
    (`self.K2_SetActorRotation` (`KismetMathLibrary.RInterpTo` (`self.K2_GetActorRotation`) (`KismetMathLibrary.MakeRotator` 0.0 (`KismetMathLibrary.FClamp` (.pitch (`KismetMathLibrary.FindLookAtRotation` (`self.K2_GetActorLocation`) (+ (`self.K2_GetActorLocation` (`self.聚集目标`)) (`self.偏移量`)))) (- _pitch 40.0) (+ _pitch 40.0)) (`KismetMathLibrary.FClamp` (.yaw (`KismetMathLibrary.FindLookAtRotation` (`self.K2_GetActorLocation`) (+ (`self.K2_GetActorLocation` (`self.聚集目标`)) (`self.偏移量`)))) (- _yaw 40.0) (+ _yaw 40.0))) 0.01 10.0))))

(fn `UserConstructionScript`)