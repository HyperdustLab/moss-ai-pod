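; Homing weapon bullet for the space game, fired by a 便便Agent at a target.
; A looping timer steers it toward the target via server-to-multicast transform events, destroying it if the shooter dies or either actor becomes invalid.
; A sphere trace triggers a one-time hit that damages a 便便Agent or 星球 (planet), with explosion VFX only for planets.
; The shooter plays launch and explosion sounds, and the bullet destroys itself shortly after impact.
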(event `self.ReceiveBeginPlay`
  (bind `_发起者` (`self.发起者`))
  (`self.服务器-设置变量` `_发起者` (`self.目标`))
  (bind `_as便便_agent` (cast `/Game/game/AI/便便Agent` `_发起者`))
  (`/Game/game/AI/便便Agent.本地-播放音效` `_as便便_agent` "/Game/game/音效/便便音效/便便攻击音效.便便攻击音效")
  (`self.服务器-设置飞行子弹`))

(event `服务器-设置变量`
  (params (`发射者` :type "Actor Object Reference") (`目标` :type "Actor Object Reference"))
  (set `self.发起者` `发射者`)
  (set `self.目标` `目标`))

(event `服务器-设置飞行子弹`
  (bind _returnvalue (`KismetSystemLibrary.K2_SetTimerDelegate` (delegate `飞行定时器`) 0.01 true))
  (set `self.NewVar` _returnvalue))

(event `服务器-变换`
  (params (NewTransform :type "Transform Structure (by ref)"))
  (`self.组播-设置变换` NewTransform))

(event `组播-设置变换`
  (params (NewTransform :type "Transform Structure (by ref)"))
  (`self.K2_SetActorTransform` NewTransform))

(event `飞行定时器`
  (bind _returnvalue (`self.K2_GetActorLocation`))
  (bind `_发起者` (`self.发起者`)
    (:`then`
      (bind `_as便便_agent` (cast `/Game/game/AI/便便Agent` `_发起者`)
        (:`then`
          (if (`/Game/game/AI/便便Agent.已死亡` `_as便便_agent`)
            (`KismetSystemLibrary.K2_ClearAndInvalidateTimerHandle` (`self.NewVar`) :!label _label)
            (`self.服务器-销毁`)
            (else
              (bind `_目标` (`self.目标` :!label _label_2)
                (:`then`
                  (`self.服务器-变换` (`KismetMathLibrary.MakeTransform` (+ (`self.K2_GetActorLocation`) (* (`self.GetActorForwardVector`) (`self.速度`))) (`KismetMathLibrary.RInterpTo` (`self.K2_GetActorRotation`) (`KismetMathLibrary.FindLookAtRotation` (`self.K2_GetActorLocation`) (`self.K2_GetActorLocation` `_目标`)) 0.01 5.0)))
                  (bind (_outhit _returnvalue_2) (`KismetSystemLibrary.SphereTraceSingleForObjects` _returnvalue _returnvalue (`self.速度`) (`|MakeArray` "ObjectTypeQuery2" "ObjectTypeQuery3" :!type "EObjectTypeQuery Enum") false (`|MakeArray` (`self.发起者`)) "ForOneFrame"))
                  (if _returnvalue_2
                    (`self.服务器-命中目标` (`.HitActor` (`GameplayStatics.BreakHitResult` _outhit)))))
                (:`else`
                  (goto _label))))))
        (:`CastFailed`
          (goto _label_2))))
    (:`else`
      (goto _label))))

(event `服务器-命中目标`
  (params (actor :type "Actor Object Reference"))
  (set `self.停止飞行` true)
  (`/Engine/EditorBlueprintResources/StandardMacros.DoOnce` false
    (:`Completed`
      (`|ExecutionSequence`
        (:`then_0`
          (bind `_as便便_agent` (cast `/Game/game/AI/便便Agent` actor)
            (:`then`
              (`/Game/game/AI/便便Agent.受伤` `_as便便_agent` 10.0))
            (:`CastFailed`
              (bind `_as星球` (cast `/Game/game/Resource_Pack/OpenSpaceShooter/Blueprints/星球` actor))
              (`/Game/game/Resource_Pack/OpenSpaceShooter/Blueprints/星球.受伤` `_as星球` 10.0 (`self.发起者`))
              (`self.组播-命中目标`))))
        (:`then_1`
          (`self.本地-命中目标`)
          (`|ExecutionSequence`
            (:`then_0`
              (`KismetSystemLibrary.Delay` 0.2)
              (`self.K2_DestroyActor`))
            (:`then_1`
              (bind `_as便便_agent_2` (cast `/Game/game/AI/便便Agent` (`self.发起者`)))
              (`/Game/game/AI/便便Agent.本地-播放音效` `_as便便_agent_2` "/Game/game/音效/便便音效/便便爆炸音效.便便爆炸音效"))))))))

(event `本地-命中目标`)

(event `组播-命中目标`
  (`NiagaraFunctionLibrary.SpawnSystemAtLocation` "/Game/ZY/fx/Lightning_Electricity_Pack/Particles/P_Explosion.P_Explosion" (`self.K2_GetActorLocation`)))

(event `服务器-销毁`
  (`self.K2_DestroyActor`))

(fn `UserConstructionScript`)