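; Treasure chest content actor (宝藏内容) that displays a web-loaded picture and reveals it when the chest is opened.
; The construction script creates dynamic instances of the painting material on Plane and Plane1.
; 设置图像 downloads an image from the given URL and, on success, sets it as both materials' texture.
; 打开宝箱 plays a timeline that scales Plane up from zero while raising the actor above its starting location.
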(event `设置图像`
  (params (`图片链接` :type String))
  (set `self.图片链接` `图片链接`)
  (bind _texture (`/Game/game/蓝图宏库.图片下载` (`self.图片链接`))
    (:`On Success`
      (`MaterialInstanceDynamic.SetTextureParameterValue` (`self.地图材质实例1`) "贴图" _texture)
      (`MaterialInstanceDynamic.SetTextureParameterValue` (`self.地图材质实例2`) "贴图" _texture))))

(event `打开宝箱`
  (bind _a (`self.A`))
  (set `self.A` (`self.K2_GetActorLocation`))
  (`|ExecutionSequence`
    (:`then_0`
      (bind (_direction `_新建轨道_0`) (`Timeline|时间轴_0` :!via `PlayFromStart`)
        (:`Update`
          (bind _returnvalue (`KismetMathLibrary.Lerp` 0.0 2.0 `_新建轨道_0`))
          (`SceneComponent.SetWorldScale3D` (`self.Plane`) (`KismetMathLibrary.MakeVector` _returnvalue _returnvalue _returnvalue))
          (`self.K2_SetActorLocation` (`KismetMathLibrary.VLerp` _a (`KismetMathLibrary.MakeVector` (.x _a) (.y _a) (+ (.z _a) 100.0)) `_新建轨道_0`)))))))

(fn `UserConstructionScript`
  (bind _returnvalue (`PrimitiveComponent.CreateDynamicMaterialInstance` (`self.Plane`) 0 "/Game/ZY/材质/材质实例/画材质_Inst.画材质_Inst" "None"))
  (set `self.地图材质实例1` _returnvalue)
  (bind _returnvalue_2 (`PrimitiveComponent.CreateDynamicMaterialInstance` (`self.Plane1`) 0 "/Game/ZY/材质/材质实例/画材质_Inst.画材质_Inst" "None"))
  (set `self.地图材质实例2` _returnvalue_2))